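; Gun actor that characters equip, fire and drop, and that players pick up or swap through an overlap prompt.
; Fire runs a multi-line trace with random aim deviation and per-surface penetration, feeding damage, impact effects and trail.
; Talks to its owner through message calls for aim, recoil and montages, updating an ammo/reticle widget for players.
; Ammo-check/auto-reload, shell and muzzle-flash activation nodes in the firing graph are disconnected.
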(event Custom|DemoShoot
  (bind _ns_flash (Variables|Default|GetNS_flash))
  (Components|Activation|Activate _ns_flash true)
  (Utilities|FlowControl|Delay 1.0)
  (Components|Activation|Deactivate _ns_flash)
  (CallFunction|DemoShoot))

(event EventBeginPlay
  (Utilities|IsValid (Actor|GetParentActor)
    (:Is%20Not%20Valid
      (CallFunction|SetInteractable true))))

(event Collision|EventActorBeginOverlap
  (params (OtherActor :type Actor%20Object%20Reference)))

(event EventTick
  (params (DeltaSeconds :type Float%20%28single-precision%29)))

(event EventDrop
  (bind _gun_mesh (Variables|Default|Getgun%20mesh))
  (CallFunction|ToggleGun false)
  (Utilities|FlowControl|Delay 0.3)
  (Transformation|DetachFromActor self "KeepWorld" "KeepWorld" "KeepWorld")
  (Collision|SetCollisionProfileName _gun_mesh "BlockAll" true :!class /Script/Engine.PrimitiveComponent)
  (Collision|SetCollisionEnabled _gun_mesh "QueryAndPhysics")
  (Physics|SetSimulatePhysics _gun_mesh true)
  (Physics|AddForce _gun_mesh "0, 0,100.000000" "None" false)
  (CallFunction|Fire false)
  (Utilities|FlowControl|Delay 3.0)
  (Physics|SetSimulatePhysics (Variables|Default|Getgun%20mesh) false)
  (CallFunction|SetInteractable true)
  (Collision|SetCollisionEnabled (Variables|Default|Getgun%20mesh) "NoCollision"))

(event EventSetInteractable
  (params (enable :type Boolean))
  (bind _player_detector (Variables|Default|Getplayer%20detector))
  (Utilities|IsValid _player_detector
    (:Is%20Valid
      (Variables|/Script/Engine.PrimitiveComponent|SetbGenerateOverlapEvents _player_detector enable))))

(event EventReloadGun
  (Variables|Default|Settotal%20ammo%20count (+ (Variables|Default|Gettotal%20ammo%20count) (Variables|Default|Getloaded%20ammo%20count)))
  (Variables|Default|Setloaded%20ammo%20count 0)
  (Variables|Default|Setloaded%20ammo%20count (Math|Integer|SelectInt (Variables|Default|Getmagazin%20capacity) (+ (Variables|Default|Gettotal%20ammo%20count) (Variables|Default|Getloaded%20ammo%20count)) (> (- (Variables|Default|Gettotal%20ammo%20count) (Variables|Default|Getmagazin%20capacity)) 0)))
  (bind _yes_no (Class|CLMBPICharacter|IsPlayer?(Message) (Variables|Default|Getcharacter)))
  (Variables|Default|Settotal%20ammo%20count (Math|Integer|SelectInt (Math|Integer|Clamp(Integer) (- (Variables|Default|Gettotal%20ammo%20count) (Variables|Default|Getmagazin%20capacity)) 0 (Variables|Default|Getmax%20ammo%20count)) (Variables|Default|Getmax%20ammo%20count) _yes_no))
  (CallFunction|UpdateAmmoCount))

(event EventSetReticleMode
  (params (reticle%20mode :type ReticleMode%20Enum :default "NewEnumerator0"))
  (bind _gun_widget (Variables|Default|Getgun%20widget)
    (:then
      (Default|SetAccuracy _gun_widget (Utilities|Select :Index reticle%20mode :NewEnumerator0 0.1 :NewEnumerator1 0.2 :NewEnumerator2 0.5)))
    (:else)))

(event EventSetReticleAccuracy
  (params (accuracy%20 :type Float%20%28double-precision%29))
  (bind _gun_widget (Variables|Default|Getgun%20widget))
  (Utilities|IsValid _gun_widget
    (:Is%20Valid
      (Default|SetAccuracy _gun_widget accuracy%20))))

(event EventAddAmmo
  (params (AmmoDelta :type Integer))
  (Variables|Default|Settotal%20ammo%20count (Math|Integer|Clamp(Integer) (+ AmmoDelta (Variables|Default|Gettotal%20ammo%20count)) 0 (Variables|Default|Getmax%20ammo%20count)))
  (CallFunction|UpdateAmmoCount))

(event Input|ActionEvents|InputActioninteract
  (params (Key :type Key%20Structure))
  (bind _unequipped_transform (Variables|Default|Getunequipped%20transform))
  (bind _gun_mesh (Variables|Default|Getgun%20mesh))
  (:Pressed
    (Transformation|SetActorLocation (Transformation|GetWorldLocation (Variables|Default|Getgun%20mesh)) false false)
    (Transformation|AttachComponentToComponent _gun_mesh (Variables|Default|GetDefaultSceneRoot) "None" "SnapToTarget" "KeepWorld" "SnapToTarget" true)
    (Components|MoveComponentTo _gun_mesh (.location _unequipped_transform) (.rotation _unequipped_transform) true true 0.2 false)
    (Class|CLMBPICharacter|SwapGun(Message) (Variables|Default|Gettarget%20character) self)
    (Input|DisableInput (Game|GetPlayerController 0))
    (CallFunction|SetInteractable false)))

(fn ConstructionScript)

(fn UpdateAmmoCount
  (bind _gun_widget (Variables|Default|Getgun%20widget))
  (Utilities|IsValid _gun_widget
    (:Is%20Valid
      (Default|UpdateAmmoCount _gun_widget (Variables|Default|Gettotal%20ammo%20count) (Variables|Default|Getloaded%20ammo%20count)))))

(fn UpdateReticle
  (params (accuracy :type Float%20%28double-precision%29))
  (CallFunction|SetReticleAccuracy accuracy))

(event EventToggleGun
  (params (equip/unequip :type Boolean) (character :type Actor%20Object%20Reference))
  (bind _gun_widget (Variables|Default|Getgun%20widget))
  (bind _equipped_transform (Variables|Default|Getequipped%20transform))
  (bind _unequipped_transform (Variables|Default|Getunequipped%20transform))
  (if (not (Class|SceneComponent|IsAnySimulatingPhysics (Variables|Default|Getgun%20mesh)))
    (bind _output_get (Variables|Default|Setcharacter character))
    (bind _aimdeviationmultiplier (Class|CLMBPICharacter|GetAimDeviationMultiplier(Message) _output_get))
    (Variables|Default|SetCharacterAimDeviationMultiplier _aimdeviationmultiplier)
    (Variables|Default|Setequipped equip/unequip)
    (if equip/unequip
      (Components|MoveComponentTo (Variables|Default|Getgun%20mesh) (.location _equipped_transform) (.rotation _equipped_transform) false false 0.2 false)
      (|GunUI)
      (CallFunction|ReloadGun)
      (else
        (Utilities|IsValid _gun_widget
          (:Is%20Valid
            (Widget|RemovefromParent _gun_widget))
          (:Is%20Not%20Valid
            _))
        (Components|MoveComponentTo (Variables|Default|Getgun%20mesh) (.location _unequipped_transform) (.rotation _unequipped_transform) false false 0.2 false)))))

(event OnComponentEndOverlap(playerdetector)
  (params (OverlappedComponent :type Primitive%20Component%20Object%20Reference) (OtherActor :type Actor%20Object%20Reference) (OtherComp :type Primitive%20Component%20Object%20Reference) (OtherBodyIndex :type Integer))
  (bind _returnvalue (Game|GetPlayerController 0))
  (bind _yes_no (Class|CLMBPICharacter|IsPlayer?(Message) OtherActor))
  (if _yes_no
    (Input|DisableInput _returnvalue)
    (Class|BPIUI|ShowTip(Message) (HUD|GetHUD _returnvalue) "" 5.0)))

(event OnComponentBeginOverlap(playerdetector)
  (params (OverlappedComponent :type Primitive%20Component%20Object%20Reference) (OtherActor :type Actor%20Object%20Reference) (OtherComp :type Primitive%20Component%20Object%20Reference) (OtherBodyIndex :type Integer) (bFromSweep :type Boolean) (SweepResult :type Hit%20Result%20Structure%20%28by%20ref%29))
  (bind _returnvalue (Game|GetPlayerController 0))
  (bind _returnvalue_2 (Game|GetPlayerController 0))
  (bind _yes_no (Class|CLMBPICharacter|IsPlayer?(Message) OtherActor))
  (if _yes_no
    (Variables|Default|Settarget%20character OtherActor)
    (Input|EnableInput (Game|GetPlayerController 0))
    (bind (_gun_type _has_weapon_from_category) (Class|CLMBPICharacter|GetWeaponfromCategory(Message) OtherActor (Variables|Default|GetGunCategory)))
    (if _has_weapon_from_category
      (bind _keys (Class|CLMBPIPlayerController|GetInput(Message) _returnvalue_2 "interact"))
      (Class|BPIUI|ShowTip(Message) (HUD|GetHUD _returnvalue_2) (Utilities|String|Append "Press <input>" _keys "</> to Swap <object>" (Utilities|String|EnumtoString _gun_type) "</> with <object>" (Utilities|String|EnumtoString (Variables|Default|GetGunType)) "</>") 5.0)
      (else
        (bind _keys_2 (Class|CLMBPIPlayerController|GetInput(Message) _returnvalue "interact"))
        (Class|BPIUI|ShowTip(Message) (HUD|GetHUD _returnvalue) (Utilities|String|Append "Press <input>" _keys_2 "</> to pickup " (Utilities|String|EnumtoString (Variables|Default|GetGunType))) 5.0)))))

(event Custom|Emit%20Bullet
  (Utilities|EmitBulletM
    (:OutputPin
      (Class|Actor|MakeNoise 1.0 0 (Transformation|GetActorLocation) (Variables|Default|GetNoise%20Range) "1"))))

(event EventFire
  (params (start/stop :type Boolean))
  (bind _ch_shoot_standing (Variables|Animations|Getch_shoot_standing))
  (bind _character (Variables|Default|Getcharacter))
  (bind _output_get (Variables|Default|Setfiring start/stop))
  (if (not (Variables|Default|Getreloading))
    (Animation|Montage|PlayMontage (Variables|Default|Getgun%20mesh) (Variables|Animations|Getgun_shoot_montage) 1.0 0.0 (select _output_get "Default" "release")
      (:then
        (Class|CLMBPICharacter|PlayCharacterMontage(Message) _character _ch_shoot_standing)
        (if (and _output_get (Variables|Default|Getequipped)) :!label _label
          (CallFunction|UpdateReticle 0.2)
          (if (Variables|Default|Getfiring)
            (Audio|PlaySoundatLocation (Variables|Default|Getshoot%20sound) (Transformation|GetActorLocation) "0, 0, 0" 1.0 1.0 0.0 0 0 0 0)
            (CallFunction|EmitBullet)
            (Math|Integer|DecrementInt (Variables|Default|Getloaded%20ammo%20count)
              (:%20%20
                (CallFunction|UpdateAmmoCount)
                (Class|CLMBPICharacter|AddRecoil(Message) (Variables|Default|Getcharacter) (Variables|Default|Getrecoil%20rotaiton) (Variables|Default|Getrecoil%20pitch%20input))
                (Variables|Default|Setrecoil%20pitch%20input (* (Variables|Default|Getrecoil%20pitch%20input) 0.8))
                (Utilities|FlowControl|Delay (Variables|Default|Getbullet_delay))
                (Components|Activation|Deactivate (Variables|Default|GetNS_flash))
                (if (Variables|Default|Getautomatic)
                  (goto _label)))))
          (else
            (if (Variables|Default|Getautomatic)
              (Class|CLMBPICharacter|StopCharacterMontage(Message) _character _ch_shoot_standing))
            (CallFunction|UpdateReticle 0.5)
            (Variables|Default|Setrecoil%20pitch%20input (Variables|Default|Getrecoil%20pitch%20input_max))))))))

(fn GetAmmoType
  (return (Variables|Default|GetAmmo%20Type)))

(fn GetBulletTarget
  (bind _target_point (Variables|Default|Gettarget%20point))
  (bind _target (Class|CLMBPICharacter|GetTargetLocation(Message) (Variables|Default|Getcharacter)))
  (bind (_outhit _returnvalue) (Collision|LineTraceByChannel (Transformation|GetSocketLocation (Variables|Default|Getgun%20mesh) "nozzle") _target "TraceTypeQuery1" false 0 "None"))
  (if _returnvalue
    (Transformation|SetRelativeLocation _target_point (Math|Vector|MakeVector (.Distance (Collision|BreakHitResult _outhit)) 0.0 0.0) false false)
    (else
      (Transformation|SetRelativeLocation _target_point (Math|Vector|MakeVector 2e+03 0.0 0.0) false false)))
  (return (Transformation|GetWorldLocation (Variables|Default|Gettarget%20point))))

(fn GetCategory
  (return (Variables|Default|GetGunCategory)))

(fn GetGunType
  (return (Variables|Default|GetGunType)))

(fn GetRange
  (return (Variables|Default|GetRange)))

(fn GetReloadAnimations
  (return (Variables|Animations|Getch_reload_standing) (Variables|Animations|Getch_reload_crouching) (Variables|Animations|Getch_reload_proning)))

(fn GetShootAnimation
  (return (Variables|Animations|Getch_shoot_standing)))

(fn GetWeaponSocket
  (params (socket%20name :type Name :default "None"))
  (return (Transformation|GetSocketTransform (Variables|Default|Getgun%20mesh) socket%20name "RTS_World")))

(fn IsEquipped
  (return (Variables|Default|Getequipped)))