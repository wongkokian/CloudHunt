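; Quest NPC "Riko" for the electricity quest, extending a parent NPC with state-indexed dialogue shown through the HUD.
; Each interaction steps through either the quest lines, with an audio cue partway, or the completion lines, depending on whether ElecQuest is complete.
; Interacting also activates the quest through a DoOnce gate.
; Ending overlap hides dialogue, resets that gate and rewinds to the relevant first line.
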(event EventBeginPlay
  (Variables|Default|SetHUDRef (Variables|/Game/UI/HUDActor.HUDActor_C|GetHUDRef (Variables|Default|GetHUDActor))))

(event EventInteract
  (Audio|Components|Audio|Stop (Variables|Default|GetAudio))
  (|CallParentFunction)
  (CallFunction|DoStuff)
  (Utilities|FlowControl|DoOnce false
    (:Completed
      (Default|ActivateQuest (Variables|Default|GetElec%20Quest))
      (Development|PrintString "Activate Quest"))))

(event Collision|EventActorEndOverlap
  (params (OtherActor :type Actor%20Object%20Reference))
  (|CallParentFunction 0)
  (Default|HideDialogue (Variables|Default|GetHUDRef))
  (if (Variables|/Game/Levels/ElectricLevel/SubQuest/BP_Quest.BP_Quest_C|GetisComplete (Variables|Default|GetElec%20Quest))
    (Variables|Default|SetState 5)
    (Utilities|FlowControl|DoOnce false) ; enters at Reset
    (else
      (Variables|Default|SetState 0)
      (Utilities|FlowControl|DoOnce false) ; enters at Reset
    )))

(fn ConstructionScript)

(fn DoStuff
  (|CallParentFunction)
  (if (Variables|/Game/Levels/ElectricLevel/SubQuest/BP_Quest.BP_Quest_C|GetisComplete (Variables|Default|GetElec%20Quest))
    (if (< (Variables|Default|GetState) 5)
      (Variables|Default|SetState 5))
    (CallFunction|PlayComplete)
    (else
      (CallFunction|PlayQuest)))
  (Math|Integer|IncrementInt (Variables|Default|GetState)))

(fn PlayQuest
  (bind _hudref (Variables|Default|GetHUDRef))
  (if (Utilities|Array|IsEmpty (Utilities|Array|Get(acopy) (Variables|Default|Getmessages) (Variables|Default|GetState)))
    (Default|HideDialogue _hudref)
    (else
      (Default|DisplayDialogue _hudref (Utilities|Array|Get(acopy) (Variables|Default|Getmessages) (Variables|Default|GetState)) (Variables|Default|GetName))))
  (switch int (Variables|Default|GetState)
    (:0
      (Variables|Default|SetName "Riko"))
    (:3
      (Audio|Components|Audio|Play (Variables|Default|GetAudio) 0.0))
    (:4
      (Variables|Default|SetState 0))))

(fn PlayComplete
  (bind _hudref (Variables|Default|GetHUDRef))
  (if (Utilities|Array|IsEmpty (Utilities|Array|Get(acopy) (Variables|Default|Getmessages) (Variables|Default|GetState)))
    (Default|HideDialogue _hudref)
    (Variables|Default|SetState 4)
    (else
      (Default|DisplayDialogue _hudref (Utilities|Array|Get(acopy) (Variables|Default|Getmessages) (Variables|Default|GetState)) (Variables|Default|GetName)))))