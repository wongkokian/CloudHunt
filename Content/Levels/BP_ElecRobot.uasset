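; BP_ElecRobot is a level robot actor whose skeletal mesh plays animations on externally triggered events.
; Trigger events for wake-up, run, jump, mid-air, land and fly rewind the mesh and play a single animation directly, looping all but jump and land.
; RemoveAnimation clears the animation and leaves a long-lasting debug print.
; GetRedBlueSpawner exposes its child-actor BP_RedBlueSpawner to callers.
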(event Custom|Trigger%20Wake%20Up
  (bind _skeletalmesh (Variables|Default|GetSkeletalMesh))
  (Components|Animation|SetPosition _skeletalmesh 0.0 true)
  (Components|Animation|PlayAnimation _skeletalmesh "/Game/Cute_Robot/Animations/Anim_Wake_Up.Anim_Wake_Up" true))

(event Custom|Trigger%20Run
  (bind _skeletalmesh (Variables|Default|GetSkeletalMesh))
  (Components|Animation|SetPosition _skeletalmesh 0.0 true)
  (Components|Animation|PlayAnimation _skeletalmesh "/Game/Cute_Robot/Animations/Anim_Sprint.Anim_Sprint" true))

(event Custom|Trigger%20Jump
  (bind _skeletalmesh (Variables|Default|GetSkeletalMesh))
  (Components|Animation|SetPosition _skeletalmesh 0.0 true)
  (Components|Animation|PlayAnimation _skeletalmesh "/Game/Cute_Robot/Animations/Anim_Run_Jump.Anim_Run_Jump" false))

(event Custom|Trigger%20Mid%20Air
  (bind _skeletalmesh (Variables|Default|GetSkeletalMesh))
  (Components|Animation|SetPosition _skeletalmesh 0.0 true)
  (Components|Animation|PlayAnimation _skeletalmesh "/Game/Cute_Robot/Animations/Anim_Jump_Middle.Anim_Jump_Middle" true))

(event Custom|Trigger%20Land
  (bind _skeletalmesh (Variables|Default|GetSkeletalMesh))
  (Components|Animation|SetPosition _skeletalmesh 0.0 true)
  (Components|Animation|PlayAnimation _skeletalmesh "/Game/Cute_Robot/Animations/Anim_Jump_Land.Anim_Jump_Land" false))

(event Custom|Trigger%20Fly
  (bind _skeletalmesh (Variables|Default|GetSkeletalMesh))
  (Components|Animation|SetPosition _skeletalmesh 0.0 true)
  (Components|Animation|PlayAnimation _skeletalmesh "/Game/Cute_Robot/Animations/Anim_Standing.Anim_Standing" true))

(event Custom|Remove%20Animation
  (Components|Animation|PlayAnimation (Variables|Default|GetSkeletalMesh) (Variables|Default|GetNull) true)
  (Development|PrintString "Hello" true true "(R=0.000000,G=0.660000,B=1.000000,A=1.000000)" 22222.0))

(event EventBeginPlay)

(event Collision|EventActorBeginOverlap
  (params (OtherActor :type Actor%20Object%20Reference)))

(event EventTick
  (params (DeltaSeconds :type Float%20%28single-precision%29)))

(fn ConstructionScript)

(fn GetRedBlueSpawner
  (bind _asbp_red_blue_spawner (Utilities|Casting|CastToBP_RedBlueSpawner (Variables|/Script/Engine.ChildActorComponent|GetChildActor (Variables|Default|GetRedBlueSpawner))))
  (return _asbp_red_blue_spawner))