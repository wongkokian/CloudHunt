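; Boss-level fire spawner that creates expanding rings of BP_Fire actors around its Center after a fixed delay from BeginPlay.
; BeginPlay spawns one fire to get its length for grid spacing and traces downward to find the ground-level center.
; A recursive, delayed event then calls SpawnFire, growing the radius each step up to MaxRadius.
; GetPointsOnCircle samples the circle by degree, rounding to integer cells and collecting them in a Set to drop duplicates.
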(event Custom|Start%20Fire%20Rings
  (CallFunction|SpawnFireRing))

(event Custom|Spawn%20Fire%20Ring
  (CallFunction|SpawnFire)
  (Utilities|FlowControl|Delay 0.5)
  (if (<= (Variables|Default|GetCurrentRadius) (Variables|Default|GetMaxRadius))
    (CallFunction|SpawnFireRing)))

(event EventBeginPlay
  (bind _center (Variables|Default|Getcenter))
  (bind _returnvalue (Transformation|GetWorldLocation _center))
  (bind _returnvalue_2 (Game|SpawnActorfromClass "/Game/Levels/Boss/FireDamage/BP_Fire.BP_Fire_C" (Transformation|GetWorldTransform (Variables|Default|Getcenter)) "Undefined" 0 0))
  (bind _len (Default|GetLength _returnvalue_2))
  (Variables|Default|Setlen _len)
  (bind _outhit (Collision|LineTraceByChannel _returnvalue (+ _returnvalue (Math|Vector|MakeVector 0.0 0.0 -1e+03)) "TraceTypeQuery1" false 0 "Persistent"))
  (Variables|Default|Setcenter_location (.location _outhit))
  (Utilities|FlowControl|Delay 17.0)
  (CallFunction|StartFireRings))

(event Collision|EventActorBeginOverlap
  (params (OtherActor :type Actor%20Object%20Reference)))

(event EventTick
  (params (DeltaSeconds :type Float%20%28single-precision%29)))

(fn ConstructionScript)

(fn GetPointsonCircle
  (params (CurrentRadius :type Integer))
  (LocalVariables|Setr CurrentRadius)
  (for _index (range 1 360)
    (Utilities|Set|Add (LocalVariables|Getpts) (Math|Vector|MakeVector (Math|Conversions|ToFloat(Integer) (Math|Float|Round (* (Math|Trig|Sin(Radians) (* (Math|Float|MultiplybyPi 2.0) (/ _index 360))) (LocalVariables|Getr)))) (Math|Conversions|ToFloat(Integer) (Math|Float|Round (* (Math|Trig|Cos(Radians) (* (Math|Float|MultiplybyPi 2.0) (/ _index 360))) (LocalVariables|Getr)))) 0.0)))
  (bind _result (Utilities|Set|ToArray (LocalVariables|Getpts)))
  (return _result))

(fn SpawnFire
  (bind _len (Variables|Default|Getlen))
  (bind _points (CallFunction|GetPointsonCircle (Variables|Default|GetCurrentRadius)))
  (for _array_element _points
    (Game|SpawnActorfromClass "/Game/Levels/Boss/FireDamage/BP_Fire.BP_Fire_C" (Math|Transform|MakeTransform (+ (Variables|Default|Getcenter_location) (* _array_element (Math|Vector|MakeVector _len _len 0.0))) "0, 0, 0" "1.000000,1.000000,1.000000") "Undefined" 0 0))
  (Math|Integer|IncrementInt (Variables|Default|GetCurrentRadius)))