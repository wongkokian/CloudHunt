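; Phase controller actor for the electric level that plays and resets a phase's Actor Sequence.
; Init caches and prints the StartLocation component's world position, and TriggerState plays the sequence.
; ResetState stops the sequence, rewinds it to StartTime, restores state, teleports the player to the cached start and sets Reseted.
; EndPhase and ActivateController are empty stubs, and the event graph runs nothing.
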(event EventBeginPlay)

(event Collision|EventActorBeginOverlap
  (params (OtherActor :type Actor%20Object%20Reference)))

(event EventTick
  (params (DeltaSeconds :type Float%20%28single-precision%29)))

(fn ConstructionScript)

(fn Init
  (bind _output_get (Variables|Default|SetStartLoc (Transformation|GetWorldLocation (Variables|Default|GetStartLocation))))
  (Development|PrintString (Utilities|String|ToString(Vector) _output_get)))

(fn ResetState
  (bind _actorsequence (Variables|Default|GetActorSequence))
  (bind _sequenceplayer (Variables|/Script/ActorSequence.ActorSequenceComponent|GetSequencePlayer _actorsequence))
  (Sequencer|Player|Stop _sequenceplayer :!class /Script/MovieScene.MovieSceneSequencePlayer)
  (Components|Timeline|SetPlaybackPosition _sequenceplayer (Utilities|Struct|MakeMovieSceneSequencePlaybackParams (Utilities|Struct|MakeFrameTime (Utilities|Struct|MakeFrameNumber 0) 0.0) (Variables|Default|GetStartTime) "" "Time" "Jump" false))
  (Class|MovieSceneSequencePlayer|RestoreState _sequenceplayer)
  (Transformation|SetActorLocation (Game|GetPlayerCharacter 0) (Variables|Default|GetStartLoc) false true)
  (Variables|Default|SetReseted true))

(fn TriggerState
  (Sequencer|Player|Play (Variables|/Script/ActorSequence.ActorSequenceComponent|GetSequencePlayer (Variables|Default|GetActorSequence)) :!class /Script/MovieScene.MovieSceneSequencePlayer))

(fn EndPhase)

(fn ActivateController)