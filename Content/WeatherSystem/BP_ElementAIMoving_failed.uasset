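; Weather element field, apparently an abandoned AI-moving variant: its sphere applies weather data to an overlapping BP_WeatherSpawner.
; Paired DoOnce gates alternate begin and end overlaps into HandelOverlap, which sets or clears weather, updates the BP_ElementDisplayer and fades music.
; While overlapped, a looping timer refreshes displayed distance and scales audio volume inversely with it.
; Spline, AI MoveTo and random-velocity movement are all disconnected, so the actor never moves itself.
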(event OnComponentHit(ElementSphere)
  (params (HitComponent :type Primitive%20Component%20Object%20Reference) (OtherActor :type Actor%20Object%20Reference) (OtherComp :type Primitive%20Component%20Object%20Reference) (NormalImpulse :type Vector :default "0, 0, 0") (Hit :type Hit%20Result%20Structure%20%28by%20ref%29)))

(event OnComponentBeginOverlap(ElementSphere)
  (params (OverlappedComponent :type Primitive%20Component%20Object%20Reference) (OtherActor :type Actor%20Object%20Reference) (OtherComp :type Primitive%20Component%20Object%20Reference) (OtherBodyIndex :type Integer) (bFromSweep :type Boolean) (SweepResult :type Hit%20Result%20Structure%20%28by%20ref%29))
  (Utilities|FlowControl|DoOnce false
    (:Completed
      (CallFunction|HandelOverlap (Variables|Default|GetOnBeginOverlap) OtherActor)
      (Utilities|FlowControl|DoOnce false) ; enters at Reset
    )))

(event OnComponentEndOverlap(ElementSphere)
  (params (OverlappedComponent :type Primitive%20Component%20Object%20Reference) (OtherActor :type Actor%20Object%20Reference) (OtherComp :type Primitive%20Component%20Object%20Reference) (OtherBodyIndex :type Integer))
  (Utilities|FlowControl|DoOnce false
    (:Completed
      (CallFunction|HandelOverlap (Variables|Default|GetOnEndOverlap) OtherActor)
      (Utilities|FlowControl|DoOnce false) ; enters at Reset
    )))

(event EventBeginPlay
  ;[1 1 1] initial the displayer
  (bind _outactors (Actor|GetAllActorsOfClass "/Game/CloudHuntBP/BP_ElementDisplayer.BP_ElementDisplayer_C"))
  (Variables|Default|SetElementDisplayer (Utilities|Array|Get(acopy) _outactors))
  ;[1 1 1] Set Origin Location
  (Variables|Default|SetOriginLocation (Transformation|GetWorldLocation (Variables|Default|GetDefaultSceneRoot))))

(event EventTick
  (params (DeltaSeconds :type Float%20%28single-precision%29)))

(fn ConstructionScript)

(fn HandelOverlap
  (params (OverlapType :type OverlapType%20Enum :default "NewEnumerator0") (OtherActor :type Actor%20Object%20Reference))
  (bind _weatherdata (Variables|Default|GetWeatherData))
  (bind _audio (Variables|Default|GetAudio))
  (bind _elementdisplayer (Variables|Default|GetElementDisplayer))
  (bind _asbp_weather_spawner (Utilities|Casting|CastToBP_WeatherSpawner OtherActor))
  (Utilities|FlowControl|Sequence
    (:then_0
      ;[1 1 1] Handle Weather Animation
      (switch Utilities|FlowControl|Switch|SwitchonOverlapType OverlapType
        (:NewEnumerator1
          (Default|SetWeatherData _asbp_weather_spawner (Variables|Default|GetWeatherData)))
        (:NewEnumerator2
          (Default|ClearWeatherData _asbp_weather_spawner (.key (Variables|Default|GetWeatherData))))))
    (:then_1
      ;[1 1 1] Handle Element Related Attributes
      (switch Utilities|FlowControl|Switch|SwitchonOverlapType OverlapType
        (:NewEnumerator1
          (Default|ModifyElement (Variables|Default|GetElementDisplayer) (.element (Variables|Default|GetWeatherData)))
          (bind _returnvalue (Utilities|Time|SetTimerbyFunctionName 0 "ModifyDisplayerDistance" 0.5 true)))
        (:NewEnumerator2
          (Default|ModifyElement _elementdisplayer (Utilities|Text|FormatText "No elemenet"))
          (Utilities|Time|ClearandInvalidateTimerbyHandle _returnvalue)
          (Default|ModifyDistance _elementdisplayer (Utilities|Text|FormatText "??")))))
    (:then_2
      ;[1 1 1] Handle Background Music
      (switch Utilities|FlowControl|Switch|SwitchonOverlapType OverlapType
        (:NewEnumerator1
          (if (Utilities|IsValid (.backgroundmusic _weatherdata))
            (Audio|Components|Audio|SetSound _audio (.backgroundmusic _weatherdata))
            (Audio|Components|Audio|FadeIn _audio 1.0 1.0 0.0 "Linear" :!class /Script/Engine.AudioComponent)))
        (:NewEnumerator2
          (Audio|Components|Audio|FadeOut (Variables|Default|GetAudio) 0.5 0.0 "Linear" :!class /Script/Engine.AudioComponent))))))

(fn ModifyDisplayerDistance
  (bind _asbp_weather_spawner (Utilities|Casting|CastToBP_WeatherSpawner (Utilities|Array|Get(acopy) (Collision|GetOverlappingActors (Variables|Default|GetElementSphere) "/Game/CloudHuntBP/WeatherSystem/BP_WeatherSpawner.BP_WeatherSpawner_C" :!class /Script/Engine.PrimitiveComponent))))
  (Default|ModifyDistance (Variables|Default|GetElementDisplayer) (Utilities|Text|ToText(Float) (|calculatedistancetoelementcenter_2_2 _asbp_weather_spawner) "HalfToEven"))
  (Audio|Components|Audio|AdjustVolume (Variables|Default|GetAudio) 0.0 (/ 1e+02 (|calculatedistancetoelementcenter_2_2 _asbp_weather_spawner)) "Linear" :!class /Script/Engine.AudioComponent))

(fn HandelMovement
  (params (DeltaSeconds :type Float%20%28double-precision%29))
  (Transformation|AddActorWorldOffset (* DeltaSeconds (Math|Vector|MakeVector (Variables|Default|GetMovingSpeedX) (Variables|Default|GetMovingSpeedY) 0.0))))