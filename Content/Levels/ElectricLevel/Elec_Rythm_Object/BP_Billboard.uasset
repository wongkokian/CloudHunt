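; BP_Billboard is an actor in the Electric level's rhythm objects that keeps itself rotated toward a camera or target actor.
; StartBillboard stores the passed reference, falling back to player 0's camera manager when it is invalid.
; It then starts a looping 0.01-second timer, in place of Tick, that sets the actor's rotation with FindLookAtRotation toward that target's location.
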(event Custom|Start%20Billboard
  (params (Target%20Reference :type Actor%20Object%20Reference))
  (CallFunction|Init Target%20Reference)
  (CallFunction|LookatPlayer)
  (Utilities|Time|SetTimerbyFunctionName 0 "LookAtPlayer" 0.01 true))

(event EventBeginPlay)

(event Collision|EventActorBeginOverlap
  (params (OtherActor :type Actor%20Object%20Reference)))

(event EventTick
  (params (DeltaSeconds :type Float%20%28single-precision%29)))

(fn ConstructionScript)

(fn LookatPlayer
  (bind _rotation (CallFunction|ReferenceRotation))
  (Transformation|SetActorRotation _rotation))

(fn Init
  (params (Target%20Reference :type Actor%20Object%20Reference))
  (if (Utilities|IsValid Target%20Reference)
    (Variables|Default|SetCamera Target%20Reference)
    (else
      (Variables|Default|SetCamera (Variables|/Script/Engine.PlayerController|GetPlayerCameraManager (Game|GetPlayerController 0))))))

(fn ReferenceRotation
  (return (Math|Rotator|FindLookatRotation (Transformation|GetActorLocation) (Transformation|GetActorLocation (Variables|Default|GetCamera)))))