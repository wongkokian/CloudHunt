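; Rhythm-game ball actor for the electric level that signals hit timing and scores how close a hit lands to its target delay.
; Start runs a timeline scaled by the delay to animate ball color, opacity, height and target ring size, then destroys the actor.
; The first Hit computes accuracy from actor age, plays explosion effects, spawns accuracy text, hides the ball and notifies PhaseController.
; A looping timer keeps it facing the player.
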(event Custom|Start
  (params (Time%20Delay :type Float%20%28double-precision%29) (Height%20Rate :type Float%20%28double-precision%29))
  (bind _rythmball (Variables|Default|GetRythmBall))
  (Variables|Default|SetTimeDelay Time%20Delay)
  (Components|Timeline|SetPlayRate (Variables|Default|GetRythm%20Indication) (/ 1.0 (* Time%20Delay 2.0)))
  (bind (_direction _color_change _alpha_change _heightchange _targetsize) (Timeline|Rythm%20Indication Play)
    (:Update
      (Rendering|Material|SetVectorParameterValueonMaterials _rythmball "Color" (Math|Vector|MakeVector (.r _color_change) (.g _color_change) (.b _color_change)))
      (Rendering|Material|SetScalarParameterValueonMaterials _rythmball "Opacity" _alpha_change)
      (Transformation|AddWorldOffset (Variables|Default|GetRythmBall) (Math|Vector|MakeVector 0.0 0.0 (* _heightchange Height%20Rate)) false false)
      (Transformation|SetRelativeScale3D (Variables|Default|GetTarget) (Math|Vector|MakeVector _targetsize _targetsize 1.0)))
    (:Finished
      (Actor|DestroyActor))
    (:DestroyTarget
      (Development|SetHiddeninGame (Variables|Default|GetTarget) true false))))

(event EventBeginPlay
  (Utilities|Time|SetTimerbyFunctionName 0 "LookAtPlayer" 0.01 true))

(event EventHit
  (Utilities|FlowControl|DoOnce false
    (:Completed
      (CallFunction|Update))))

(fn ConstructionScript)

(fn UpdateController
  (Default|UpdateNumHit (Variables|Default|GetPhaseController)))

(fn CalculateAccuracy
  (bind _timedelay (Variables|Default|GetTimeDelay))
  ;[1 1 1] Accuracy = elapsed time
  (return (- 1.0 (/ (Math|Float|Absolute(Float) (- (Actor|GetGameTimeSinceCreation) _timedelay)) _timedelay))))

(fn Update
  (bind _returnvalue (Transformation|GetActorLocation))
  (bind _accuracy (CallFunction|CalculateAccuracy))
  (LocalVariables|SetAccuracy _accuracy)
  (Effects|SpawnEmitteratLocation "/Game/StarterContent/Particles/P_Explosion.P_Explosion" _returnvalue "0, 0, 0" "2.000000,2.000000,2.000000")
  (Audio|SpawnSoundatLocation "/Game/StarterContent/Audio/Explosion01.Explosion01" _returnvalue "0, 0, 0" 1.0 1.0 0.0 0 0)
  (bind _returnvalue_2 (Game|SpawnActorfromClass "/Game/Levels/ElectricLevel/Elec_Rythm_Object/BP_RythmAccFB.BP_RythmAccFB_C" (Math|Transform|MakeTransform _returnvalue "0, 0, 0" "1.000000,1.000000,1.000000") "Undefined" 0 0))
  (Default|UpdateText _returnvalue_2 (LocalVariables|GetAccuracy))
  (Rendering|SetActorHiddenInGame true)
  (CallFunction|UpdateController))

(fn LookatPlayer
  (bind _returnvalue (Transformation|GetActorLocation))
  (bind _returnvalue_2 (Game|GetPlayerCharacter 0))
  (bind _returnvalue_3 (Transformation|GetActorLocation _returnvalue_2))
  (bind _returnvalue_4 (Math|Rotator|FindLookatRotation _returnvalue _returnvalue_3))
  (Transformation|SetActorRotation (Math|Rotator|MakeRotator (.roll _returnvalue_4) (.pitch _returnvalue_4) (.yaw _returnvalue_4))))