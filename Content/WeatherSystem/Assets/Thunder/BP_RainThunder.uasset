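; Weather actor that keeps Niagara-style rain above the player and stages random lightning strikes.
; Tick moves the detached rain component over the player character.
; A looping timer relocates the actor ahead of the camera facing the player, picks one of two bolt textures, plays thunder and animates the plane material through a timeline.
; Each strike briefly switches the post-process volume to manual exposure for a screen flash, requiring that volume be set.
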(event Custom|Strike
  (bind _thunder_plane (Variables|Default|GetThunder_plane))
  (|ReLocate
    (:OutputPin
      (|ChangeTexture
        (:OutputPin
          (Audio|PlaySound2D "/Game/Audio/SW_LightningStrike.SW_LightningStrike" 1.0 1.0 0.0 0 0)
          (bind _y (Timeline|Thunder_strike PlayFromStart)
            (:Update
              (Rendering|Material|SetScalarParameterValueonMaterials _thunder_plane "Y" _y)
              (Rendering|Material|SetScalarParameterValueonMaterials _thunder_plane "emission" (* (+ _y 1.0) 2e+01)))))))))

(event EventBeginPlay
  (bind _pp_volume (Variables|Default|GetPP_volume))
  (Transformation|DetachFromComponent (Variables|Default|GetNS_Rain) "KeepRelative" "KeepWorld" "KeepWorld" true)
  (Utilities|IsValid (Variables|Default|GetPP_volume)
    (:Is%20Valid
      (Utilities|FlowControl|Delay (Math|Random|RandomFloatinRange 6.0 8.0) :!label _label)
      (CallFunction|Strike)
      (Utilities|FlowControl|Delay 0.2)
      (bind _output_get (Variables|Default|SetOriginal%20Exposure%20Compensation (Utilities|Struct|BreakPostProcessSettings (Variables|/Script/Engine.PostProcessVolume|GetSettings _pp_volume))))
      (Variables|/Script/Engine.PostProcessVolume|SetSettings _pp_volume (Utilities|Struct|MakePostProcessSettings "AEM_Manual" 16.0))
      (Utilities|FlowControl|Delay 0.2)
      (Variables|/Script/Engine.PostProcessVolume|SetSettings _pp_volume (Utilities|Struct|MakePostProcessSettings "AEM_Histogram" _output_get))
      (goto _label))
    (:Is%20Not%20Valid
      (Development|PrintString "No post process volume set " true true "(R=1.000000,G=0.155378,B=0.000000,A=1.000000)" 1e+01))))

(event Collision|EventActorBeginOverlap
  (params (OtherActor :type Actor%20Object%20Reference)))

(event EventTick
  (params (DeltaSeconds :type Float%20%28single-precision%29))
  (Transformation|SetWorldLocation (Variables|Default|GetNS_Rain) (+ (Transformation|GetActorLocation (Game|GetPlayerCharacter 0)) "0,0,1000.000000") false false))

(fn ConstructionScript)