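; BP_RedBlueBall is a ball actor in the electric rhythm-ball level that homes in on the player character.
; A looping 0.01-second timer started at BeginPlay calls MoveToPlayer, which steps the Ball component by Speed toward the player's current location.
; Movement teleports without sweep, and the actor destroys itself once its age reaches TimeDelay.
; Overlap, hit and Tick events are empty.
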(event OnComponentHit(Ball)
  (params (HitComponent :type Primitive%20Component%20Object%20Reference) (OtherActor :type Actor%20Object%20Reference) (OtherComp :type Primitive%20Component%20Object%20Reference) (NormalImpulse :type Vector :default "0, 0, 0") (Hit :type Hit%20Result%20Structure%20%28by%20ref%29)))

(event EventBeginPlay
  (Utilities|Time|SetTimerbyFunctionName 0 "MoveToPlayer" 0.01 true))

(event Collision|EventActorBeginOverlap
  (params (OtherActor :type Actor%20Object%20Reference)))

(event EventTick
  (params (DeltaSeconds :type Float%20%28single-precision%29)))

(fn ConstructionScript)

(fn MovetoPlayer
  (bind _ball (Variables|Default|GetBall))
  (bind _returnvalue (Transformation|GetWorldLocation _ball))
  (if (>= (Actor|GetGameTimeSinceCreation) (Variables|Default|GetTimeDelay))
    (Actor|DestroyActor)
    (else
      (Transformation|SetWorldLocation (Variables|Default|GetBall) (+ (* (Math|Vector|GetUnitDirection(Vector) _returnvalue (Transformation|GetActorLocation (Game|GetPlayerCharacter 0))) (Variables|Default|GetSpeed)) _returnvalue) false true))))