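; BP_Thunder is a telegraphed lightning strike hazard actor: a cloud with a ground indicator.
; On BeginPlay a downward trace places the indicator, then the Effect timeline drives both materials' Alpha.
; Its Strike event spawns Niagara lightning, hides the indicator and sphere-traces down for ALS_Player; hits and first overlap only print "Hit".
; When the timeline finishes, the actor hides and destroys itself after a short delay.
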(event EventBeginPlay
  (bind _returnvalue (Transformation|GetActorLocation))
  (Rendering|Material|SetScalarParameterValueonMaterials (Variables|Default|Getindicator) "Emission" 1.0)
  (bind _outhit (Collision|LineTraceByChannel _returnvalue (- _returnvalue "0.000000,0.000000,10000.000000") "TraceTypeQuery1" false (Utilities|Array|MakeArray (Game|GetPlayerCharacter 0)) "None"))
  (Transformation|SetWorldLocation (Variables|Default|Getindicator) (.location _outhit) false false)
  (bind _alpha (Timeline|Effect Play)
    (:Update
      (Rendering|Material|SetScalarParameterValueonMaterials (Variables|Default|Getcloud) "Alpha" _alpha)
      (Rendering|Material|SetScalarParameterValueonMaterials (Variables|Default|Getindicator) "Alpha" _alpha))
    (:Finished
      (Rendering|SetActorHiddenInGame true)
      (Utilities|FlowControl|Delay 2.0)
      (Actor|DestroyActor))
    (:Strike
      (Niagara|SpawnSystematLocation "/Game/Levels/Boss/ElectricDamage/Lightning/NS_Lightning.NS_Lightning" (Transformation|GetActorLocation))
      (CallFunction|CheckforPlayer)
      (Development|SetHiddeninGame (Variables|Default|Getindicator) true false))))

(event Collision|EventActorBeginOverlap
  (params (OtherActor :type Actor%20Object%20Reference))
  (Utilities|FlowControl|DoOnce false
    (:Completed
      (Development|PrintString "Hit"))))

(event EventTick
  (params (DeltaSeconds :type Float%20%28single-precision%29)))

(fn ConstructionScript)

(fn CheckforPlayer
  (bind _returnvalue (Transformation|GetActorLocation))
  (bind _outhit (Collision|SphereTraceByChannel _returnvalue (- _returnvalue "0,0,1000.000000") 2e+02 "TraceTypeQuery1" false 0 "None"))
  (if (== (Utilities|GetClass (.hitactor _outhit)) "/Game/AdvancedLocomotionV4/Blueprints/CharacterLogic/ALS_Player.ALS_Player_C")
    (Development|PrintString "Hit")))