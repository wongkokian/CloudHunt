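; BP_SmokeGrenade is a grenade Blueprint that releases a timed smoke cloud with a whistle sound.
; It extends the parent's explode event to start Niagara smoke and audio, then after a short delay enables a query-only sphere and emits noise at the grenade mesh.
; When the smoke duration ends, it stops the effect, fades the sound, disables the sphere and sets a short lifespan for cleanup.
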(event EventBeginPlay
  (|CallParentFunction)
  (Variables|Default|SetLifespan (+ (Variables|Default|GetSmokeDuration) 5.0))
  (Collision|SetCollisionEnabled (Variables|Default|GetSphere) "NoCollision"))

(event Collision|EventActorBeginOverlap
  (params (OtherActor :type Actor%20Object%20Reference))
  (|CallParentFunction OtherActor) ; This node is disabled and will not be called.\nDrag off pins to build functionality.
)

(event EventTick
  (params (DeltaSeconds :type Float%20%28single-precision%29))
  (|CallParentFunction DeltaSeconds) ; This node is disabled and will not be called.\nDrag off pins to build functionality.
)

(event EventExplodeGrenade
  (|CallParentFunction)
  (Components|Activation|Activate (Variables|Default|GetNS_Smoke) false)
  (Components|Activation|Activate (Variables|Default|GetSmokeWhistle) false)
  (Utilities|FlowControl|Delay 3.0)
  (Collision|SetCollisionEnabled (Variables|Default|GetSphere) "QueryOnly")
  (Class|Actor|MakeNoise 1.0 0 (Transformation|GetWorldLocation (Variables|Default|GetSM%20Grenade)) 1e+03 "None")
  (Utilities|FlowControl|Delay (Variables|Default|GetSmokeDuration))
  (Components|Activation|Deactivate (Variables|Default|GetNS_Smoke))
  (Audio|Components|Audio|FadeOut (Variables|Default|GetSmokeWhistle) 1.0 0.0 "Linear" :!class /Script/Engine.AudioComponent)
  (Collision|SetCollisionEnabled (Variables|Default|GetSphere) "NoCollision")
  (Actor|SetLifeSpan 5.0))

(fn ConstructionScript
  (|CallParentFunction))