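; Phase controller for the car section of the Elec3 electric level, where sequencer events drop cars by index, boost player jump and movement, and complete the phase.
; Resetting the phase respawns and starts the cars through CarSpawner.
; Overlapping the End trigger restores player gravity and sets IsComplete, with its collision toggled on activation and deactivation.
; Lifecycle functions extend a parent controller, and accuracy always reports full.
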(event OnComponentBeginOverlap(End)
  (params (OverlappedComponent :type Primitive%20Component%20Object%20Reference) (OtherActor :type Actor%20Object%20Reference) (OtherComp :type Primitive%20Component%20Object%20Reference) (OtherBodyIndex :type Integer) (bFromSweep :type Boolean) (SweepResult :type Hit%20Result%20Structure%20%28by%20ref%29))
  (bind _asals_player (Utilities|Casting|CastToALS_Player OtherActor))
  (Variables|/Script/Engine.CharacterMovementComponent|SetGravityScale (Variables|/Script/Engine.Character|GetCharacterMovement _asals_player) 1.0)
  (Utilities|FlowControl|DoOnce false :!label _label
    (:Completed
      (Variables|Default|SetisComplete true)
      (goto _label Reset))))

(event EventBeginPlay
  (CallFunction|Init))

(event Collision|EventActorBeginOverlap
  (params (OtherActor :type Actor%20Object%20Reference)))

(event EventTick
  (params (DeltaSeconds :type Float%20%28single-precision%29)))

(event Custom|SequenceEvent_0
  (Development|PrintString "Last Jump"))

(event Custom|Complete%20Car
  (CallFunction|Complete))

(event Custom|Set%20High%20Jump
  (bind _electriclevelcontroller (Variables|Default|GetElectricLevelController))
  (Default|SetPlayerJump _electriclevelcontroller 1.25e+03 3e+01 2.5)
  (Default|SetPlayerMovement _electriclevelcontroller 1.2e+03 5.0))

(event Custom|SequenceEvent_1
  (Development|PrintString "Second last"))

(event Custom|Drop%20Car
  (params (Car%20Index :type Integer))
  (Default|DropCar (Utilities|Array|Get(acopy) (Variables|/Game/Levels/ElectricLevel/Spawner/BP_CarSpawner.BP_CarSpawner_C|GetCars (Variables|Default|GetCarSpawner)) Car%20Index)))

(fn ConstructionScript)

(fn TriggerPhase
  (|CallParentFunction))

(fn Init
  (|CallParentFunction))

(fn ResetPhase
  (bind _carspawner (Variables|Default|GetCarSpawner))
  (Default|RemoveCar _carspawner)
  (Default|SpawnCar _carspawner 15.7)
  (Default|StartCar _carspawner)
  (CallFunction|EnableCollision)
  (|CallParentFunction))

(fn EnableCollision
  (Collision|SetCollisionEnabled (Variables|Default|GetEnd) "QueryOnly"))

(fn DisableCollision
  (Collision|SetCollisionEnabled (Variables|Default|GetEnd) "NoCollision"))

(fn GetAccuracy
  (return 1e+02))

(fn ActivateController
  (CallFunction|EnableCollision)
  (|CallParentFunction))

(fn DeactivateController
  (CallFunction|DisableCollision)
  (|CallParentFunction))

(fn EndPhase
  (|CallParentFunction))