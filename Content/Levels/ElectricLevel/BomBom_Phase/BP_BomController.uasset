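; BP_BomController runs the BomBom phase of the Electric level, extending a parent phase controller's lifecycle.
; Sequencer events tell the Spawner to spawn beat-indexed boms with per-beat delay and height, and handle completion and a scripted player jump.
; Player overlap with OutOfBound resets the level controller's current state, while End marks completion.
; Phase resets clear balls and re-enable both triggers; accuracy comes from the Spawner.
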(event OnComponentBeginOverlap(OutOfBound)
  (params (OverlappedComponent :type Primitive%20Component%20Object%20Reference) (OtherActor :type Actor%20Object%20Reference) (OtherComp :type Primitive%20Component%20Object%20Reference) (OtherBodyIndex :type Integer) (bFromSweep :type Boolean) (SweepResult :type Hit%20Result%20Structure%20%28by%20ref%29))
  (Development|PrintString "Hello")
  (if (== (Utilities|GetClass OtherActor) "/Game/AdvancedLocomotionV4/Blueprints/CharacterLogic/ALS_Player.ALS_Player_C")
    (Utilities|FlowControl|DoOnce false :!label _label
      (:Completed
        (CallFunction|OverlapOutOfBound)
        (Development|PrintString "RESEETTTTTT")
        (goto _label Reset)))))

(event OnComponentBeginOverlap(End)
  (params (OverlappedComponent :type Primitive%20Component%20Object%20Reference) (OtherActor :type Actor%20Object%20Reference) (OtherComp :type Primitive%20Component%20Object%20Reference) (OtherBodyIndex :type Integer) (bFromSweep :type Boolean) (SweepResult :type Hit%20Result%20Structure%20%28by%20ref%29))
  (Development|PrintString "Hello")
  (if (== (Utilities|GetClass OtherActor) "/Game/AdvancedLocomotionV4/Blueprints/CharacterLogic/ALS_Player.ALS_Player_C")
    (Utilities|FlowControl|DoOnce false :!label _label
      (:Completed
        (Variables|Default|SetisComplete true)
        (goto _label Reset)))))

(event EventBeginPlay
  (CallFunction|Init))

(event EventTick
  (params (DeltaSeconds :type Float%20%28single-precision%29)))

(event Custom|Spawn
  (bind _beatcounter (Variables|Default|GetBeatCounter))
  (Default|SpawnBom (Variables|Default|GetSpawner) (Utilities|Array|Get(acopy) (Variables|Default|GetBeatTime) _beatcounter) (Utilities|Array|Get(acopy) (Variables|Default|GetHeigtRate) _beatcounter))
  (Math|Integer|IncrementInt _beatcounter))

(event Custom|Remove%20Bound%20Check
  (Collision|SetCollisionEnabled (Variables|Default|GetOutOfBound) "NoCollision"))

(event Custom|Jump
  (bind _playercharacter (Variables|Default|GetPlayerCharacter))
  (bind _charactermovement (Variables|/Script/Engine.Character|GetCharacterMovement _playercharacter))
  (Variables|/Script/Engine.CharacterMovementComponent|SetMaxWalkSpeed _charactermovement 1525.0)
  (Variables|/Script/Engine.CharacterMovementComponent|SetMinAnalogWalkSpeed _charactermovement 8e+02)
  (Variables|/Script/Engine.CharacterMovementComponent|SetGravityScale _charactermovement 1.25)
  (AI|Navigation|SimpleMovetoLocation (Game|GetPlayerController 0) (Math|Vector|MakeVector 1.156e+04 1.927e+04 4.58e+03)))

(event Custom|Complete%20Bom
  (CallFunction|Complete))

(event Custom|Enable%20Input
  (Input|SetIgnoreMoveInput (Game|GetPlayerController 0) false))

(fn ConstructionScript)

(fn Init
  (Variables|/Game/Levels/ElectricLevel/Spawner/BP_Spawner.BP_Spawner_C|SetPhaseController (Variables|Default|GetSpawner) self)
  (|CallParentFunction))

(fn ResetPhase
  (Variables|Default|SetBeatCounter 0)
  (CallFunction|EnableCollision)
  (Default|RemoveAllBalls (Variables|Default|GetSpawner))
  (|CallParentFunction))

(fn OverlapOutOfBound
  (Default|ResetCurrentState (Variables|Default|GetElectricLevelController)))

(fn TriggerPhase
  (|CallParentFunction))

(fn EndPhase
  (|CallParentFunction)
  (Default|ResetAccuracy (Variables|Default|GetSpawner)))

(fn GetAccuracy
  (bind _average_accuray (Default|GetAverageAccuracy (Variables|Default|GetSpawner)))
  (return _average_accuray))

(fn DeactivateController
  (CallFunction|DisableCollision)
  (|CallParentFunction))

(fn ActivateController
  (CallFunction|ResetPhase)
  (|CallParentFunction))

(fn EnableCollision
  (Collision|SetCollisionEnabled (Variables|Default|GetEnd) "QueryOnly")
  (Collision|SetCollisionEnabled (Variables|Default|GetOutOfBound) "QueryOnly"))

(fn DisableCollision
  (Collision|SetCollisionEnabled (Variables|Default|GetEnd) "NoCollision")
  (Collision|SetCollisionEnabled (Variables|Default|GetOutOfBound) "NoCollision"))