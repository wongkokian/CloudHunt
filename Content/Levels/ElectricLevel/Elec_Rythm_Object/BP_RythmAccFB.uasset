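; BP_RythmAccFB is a short-lived floating text actor that shows accuracy feedback, apparently for the electric level's rhythm mechanic.
; UpdateText maps an accuracy value to an entry in AccuracyTexts by scaled, floored index, using the last entry when the scaled value is zero or less.
; It then destroys itself after a delay.
; Each Tick rotates the whole actor to face the player character.
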(event Custom|UpdateText
  (params (Acc :type Float%20%28double-precision%29))
  (CallFunction|Acc2Text Acc)
  (Utilities|FlowControl|Delay (Variables|Default|GetDuration))
  (Actor|DestroyActor))

(event EventBeginPlay)

(event Collision|EventActorBeginOverlap
  (params (OtherActor :type Actor%20Object%20Reference)))

(event EventTick
  (params (DeltaSeconds :type Float%20%28single-precision%29))
  (Transformation|SetActorRotation (Math|Rotator|FindLookatRotation (Transformation|GetActorLocation) (Transformation|GetActorLocation (Game|GetPlayerCharacter 0)))))

(fn ConstructionScript)

(fn Acc2Text
  (params (Acc :type Float%20%28double-precision%29))
  (bind _text (Variables|Default|Gettext))
  (bind _accuracytexts (Variables|Default|GetAccuracyTexts))
  (bind _accuracytexts_2 (Variables|Default|GetAccuracyTexts))
  (bind _returnvalue (Utilities|Array|Length _accuracytexts_2))
  (bind _returnvalue_2 (- _returnvalue 1))
  (bind _returnvalue_3 (* Acc _returnvalue_2))
  (if (> _returnvalue_3 0.0)
    (Rendering|Components|TextRender|SetText _text (Utilities|Array|Get(acopy) _accuracytexts (Math|Float|Floor _returnvalue_3)))
    (else
      (Rendering|Components|TextRender|SetText _text (Utilities|Array|Get(acopy) _accuracytexts _returnvalue_2)))))