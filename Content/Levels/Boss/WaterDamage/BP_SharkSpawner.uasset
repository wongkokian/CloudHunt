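; Boss-level water hazard spawner that holds a volley of BP_SharkDamage actors and fires them at the player one at a time.
; Init spawns and attaches a shark at each of four marker components, all sharing the fourth marker's rotation.
; ShootShark fires the shark at the current counter with a given delay, working backwards through the array without refilling.
; A recursive timed test loop exists, but its Init-and-start chain is unconnected.
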(event Custom|Test%20Shoot%20Shark
  (CallFunction|ShootShark 2.0)
  (Utilities|FlowControl|Delay 2.0)
  (if (>= (Variables|Default|Getcounter) 0)
    (CallFunction|TestShootShark)))

(event Custom|Shoot%20Shark
  (params (delay :type Float%20%28double-precision%29))
  (if (>= (Variables|Default|Getcounter) 0)
    (Default|ShootatPlayer (Utilities|Array|Get(acopy) (Variables|Default|GetSharks) (Variables|Default|Getcounter)) delay)
    (Math|Integer|DecrementInt (Variables|Default|Getcounter))))

(event EventBeginPlay)

(event Collision|EventActorBeginOverlap
  (params (OtherActor :type Actor%20Object%20Reference)))

(event EventTick
  (params (DeltaSeconds :type Float%20%28single-precision%29)))

(fn ConstructionScript)

(fn Init
  (bind _locations (LocalVariables|GetLocations))
  (Utilities|Array|Add _locations (Transformation|GetWorldLocation (Variables|Default|Get1)))
  (Utilities|Array|Add _locations (Transformation|GetWorldLocation (Variables|Default|Get2)))
  (Utilities|Array|Add _locations (Transformation|GetWorldLocation (Variables|Default|Get3)))
  (Utilities|Array|Add _locations (Transformation|GetWorldLocation (Variables|Default|Get4)))
  (for _array_element (LocalVariables|GetLocations)
    (bind _returnvalue (Game|SpawnActorfromClass "/Game/Levels/Boss/WaterDamage/BP_SharkDamage.BP_SharkDamage_C" (Math|Transform|MakeTransform _array_element (Transformation|GetWorldRotation (Variables|Default|Get4)) "1.000000,1.000000,1.000000") "Undefined" 0 0))
    (Utilities|Array|Add (LocalVariables|Gets) _returnvalue)
    (Transformation|AttachActorToActor _returnvalue self "None" "KeepWorld" "KeepWorld" "KeepWorld" true))
  (bind _output_get (Variables|Default|SetSharks (LocalVariables|Gets)))
  (Variables|Default|Setcounter (- (Utilities|Array|Length _output_get) 1)))