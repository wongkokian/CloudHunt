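; BP_BlueTrace is an ElectricLevel actor that moves along a supplied array of transforms, then destroys itself.
; Init stores the transforms, sample count, duration and lane position, and Start launches a looping timer at duration divided by sample count.
; Each Move tick snaps to the next transform without sweeping, shifts along local Y by the lane position, and destroys the actor once the counter exceeds the sample count.
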(event Custom|Start
  (Utilities|Time|SetTimerbyFunctionName 0 "Move" (/ (Variables|Default|GetTime) (Variables|Default|GetSampleRate)) true))

(event EventBeginPlay)

(event Collision|EventActorBeginOverlap
  (params (OtherActor :type Actor%20Object%20Reference)))

(event EventTick
  (params (DeltaSeconds :type Float%20%28single-precision%29)))

(fn ConstructionScript)

(fn Move
  (bind _counter (Variables|Default|GetCounter))
  (Transformation|SetActorTransform (Utilities|Array|Get(acopy) (Variables|Default|GetTransform) _counter))
  (Transformation|AddActorLocalOffset (Math|Vector|MakeVector 0.0 (Math|Conversions|ToFloat(Integer) (* (- (Variables|Default|GetPosition) 1) 500)) 0.0) false false)
  (bind _result (Math|Integer|IncrementInt _counter)
    (:%20%20
      (if (not (<= _result (Variables|Default|GetSampleRate)))
        (Actor|DestroyActor)))))

(fn Init
  (params (Transforms :type Array%20of%20Transforms) (SampleRates :type Integer) (Time :type Float%20%28double-precision%29) (Position :type Integer))
  (Variables|Default|SetTransform Transforms)
  (Variables|Default|SetSampleRate SampleRates)
  (Variables|Default|SetTime Time)
  (Variables|Default|SetPosition Position))