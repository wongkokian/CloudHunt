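; Boss level spawner that rains BP_Thunder strikes around and onto the player.
; Two looping timers start on BeginPlay: a frequent one for scattered strikes and a slower one for strikes at the player's position.
; Scattered strikes take a random angle and separately randomized X and Y distances within Radius of the player.
; All strikes spawn at the spawner's own height, and the SpawnThunder sequencer event is empty.
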(event EventBeginPlay
  (Utilities|Time|SetTimerbyFunctionName 0 "SpawnRandomThunder" 0.4 true)
  (Utilities|Time|SetTimerbyFunctionName 0 "SpawnThunderOnPlayer" 1.6 true))

(event Collision|EventActorBeginOverlap
  (params (OtherActor :type Actor%20Object%20Reference)))

(event EventTick
  (params (DeltaSeconds :type Float%20%28single-precision%29)))

(event Custom|Spawn%20Thunder)

(fn ConstructionScript)

(fn SpawnRandomThunder
  (bind _returnvalue (Math|Random|RandomFloat))
  (bind _returnvalue_2 (Game|GetPlayerCharacter 0))
  (bind _returnvalue_3 (Math|Random|RandomFloat))
  (bind _radius (Variables|Default|GetRadius))
  (bind _returnvalue_4 (Transformation|GetActorLocation _returnvalue_2))
  (bind _returnvalue_5 (* _radius _returnvalue_3))
  (LocalVariables|Settheta (Math|Random|RandomFloatinRange 0.0 6.28))
  (Game|SpawnActorfromClass "/Game/Levels/Boss/ElectricDamage/BP_Thunder.BP_Thunder_C" (Math|Transform|MakeTransform (Math|Vector|MakeVector (- (.x _returnvalue_4) (* (Math|Trig|Cos(Radians) (LocalVariables|Gettheta)) _returnvalue_5)) (- (.y _returnvalue_4) (* (Math|Trig|Sin(Radians) (LocalVariables|Gettheta)) _returnvalue_5)) (.z (Transformation|GetActorLocation))) (Math|Rotator|MakeRotator _returnvalue _returnvalue 0.0) "1.000000,1.000000,1.000000") "Undefined" 0 0))

(fn SpawnThunderonPlayer
  (bind _returnvalue (Game|GetPlayerCharacter 0))
  (bind _returnvalue_2 (Transformation|GetActorLocation _returnvalue))
  (Game|SpawnActorfromClass "/Game/Levels/Boss/ElectricDamage/BP_Thunder.BP_Thunder_C" (Math|Transform|MakeTransform (Math|Vector|MakeVector (.x _returnvalue_2) (.y _returnvalue_2) (.z (Transformation|GetActorLocation))) "0, 0, 0" "1.000000,1.000000,1.000000") "Undefined" 0 0))