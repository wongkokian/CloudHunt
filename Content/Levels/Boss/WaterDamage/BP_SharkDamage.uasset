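; BP_SharkDamage is a shark projectile that, when told to shoot, lunges at the player character's position captured at that moment.
; ShootAtPlayer orients the shark along the player-to-shark line, then MoveToTarget spawns a BP_SharkIndicator at that spot.
; A timeline, rate-scaled by Delay, sweeps the shark there while scaling the flat indicator.
; Arrival or any overlap plays a splash and destroys both actors; overlap only prints a hit, applying no damage.
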(event Custom|Move%20To%20Target
  (bind _returnvalue (Game|SpawnActorfromClass "/Game/Levels/Boss/WaterAttack/BP_SharkIndicator.BP_SharkIndicator_C" (Math|Transform|MakeTransform (Variables|Default|GetLocation) "0, 0, 0" "1.000000,1.000000,1.000000") "Undefined" 0 0))
  (Variables|Default|Setind _returnvalue)
  (Components|Timeline|SetPlayRate (Variables|Default|GetMove) (/ 1.0 (Variables|Default|GetDelay)))
  (bind (_direction _alpha _scale) (Timeline|Move Play)
    (:Update
      (Transformation|SetActorLocation (Math|Vector|Lerp(Vector) (Variables|Default|GetOriginalLoc) (Variables|Default|GetLocation) _alpha) true false)
      (Transformation|SetWorldScale3D (Variables|/Game/Levels/Boss/WaterAttack/BP_SharkIndicator.BP_SharkIndicator_C|Getindicator (Variables|Default|Getind)) (Math|Vector|MakeVector _scale _scale 0.01)))
    (:Finished
      (CallFunction|DestroyShark))))

(event Custom|Shoot%20At%20Player
  (params (Delay :type Float%20%28double-precision%29))
  (Variables|Default|SetDelay Delay)
  (CallFunction|LockonTarget)
  (Variables|Default|SetOriginalLoc (Transformation|GetActorLocation))
  (CallFunction|MovetoTarget))

(event EventBeginPlay
  (Components|Animation|PlayAnimation (Variables|Default|GetShark) "/Game/WaterElements/great-white-shark/source/shark_Anim_Shark_Armature_Swim.shark_Anim_Shark_Armature_Swim" true))

(event Collision|EventActorBeginOverlap
  (params (OtherActor :type Actor%20Object%20Reference))
  (Development|PrintString "Hit player")
  (CallFunction|DestroyShark))

(event EventTick
  (params (DeltaSeconds :type Float%20%28single-precision%29)))

(fn ConstructionScript)

(fn LockonTarget
  (bind _returnvalue (Game|GetPlayerCharacter 0))
  (bind _mesh (Variables|/Script/Engine.Character|GetMesh _returnvalue))
  (bind _returnvalue_2 (Transformation|GetWorldLocation _mesh))
  (Transformation|SetActorRotation (Math|Conversions|RotationFromXVector (Math|Vector|GetUnitDirection(Vector) _returnvalue_2 (Transformation|GetActorLocation))))
  (Variables|Default|SetLocation _returnvalue_2))

(fn DestroyShark
  (Audio|PlaySoundatLocation "/Game/Levels/Boss/WaterDamage/Water-Splash.Water-Splash" (Transformation|GetActorLocation) "0, 0, 0" 1.5 1.0 0.5 0 0 0 0)
  (Actor|DestroyActor)
  (Actor|DestroyActor (Variables|Default|Getind)))