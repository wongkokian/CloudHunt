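; Timed bubble for the boss water attack that the player touches to damage the Boss.
; StartBubble enables query collision, starts camera billboarding and plays a timeline over twice the Delay, scaling the plane and moving the bubble vertically.
; Player overlap plays a hit sound and deals damage scaled by timing accuracy, peaking at Delay after start.
; A hit or timeline completion destroys the bubble and all its siblings.
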(event Custom|Start%20Bubble
  (params (Delay :type Float%20%28double-precision%29))
  (bind _originallocation (Variables|Default|GetOriginalLocation))
  (Collision|SetCollisionEnabled (Variables|Default|GetBubble) "QueryOnly")
  (Variables|Default|SetDelay Delay)
  (CallFunction|SetStartTime)
  (CallFunction|StartBillboard (Game|GetPlayerCameraManager 0))
  (Components|Timeline|SetPlayRate (Variables|Default|GetBubble%20Movement) (/ 1.0 (* (Variables|Default|GetDelay) 2.0)))
  (bind (_direction _scale _heightrate) (Timeline|Bubble%20Movement Play)
    (:Update
      (Transformation|SetWorldScale3D (Variables|Default|GetPlane) (Math|Vector|MakeVector (* _scale (Variables|Default|GetTargetOriginalScale)) (* _scale (Variables|Default|GetTargetOriginalScale)) 1.0))
      (Transformation|SetWorldLocation (Variables|Default|GetDefaultSceneRoot) (Math|Vector|MakeVector (.x _originallocation) (.y _originallocation) (+ (* _heightrate (Variables|Default|GetMaxHeight)) (.z _originallocation))) false false))
    (:Finished
      (CallFunction|Destroy))))

(event EventBeginPlay
  (Variables|Default|SetTargetOriginalScale (.x (Transformation|GetWorldScale (Variables|Default|GetPlane))))
  (Variables|Default|SetOriginalLocation (Transformation|GetActorLocation)))

(event Collision|EventActorBeginOverlap
  (params (OtherActor :type Actor%20Object%20Reference))
  (if (== (Utilities|GetClass OtherActor) "/Game/AdvancedLocomotionV4/Blueprints/CharacterLogic/ALS_Player.ALS_Player_C")
    (Utilities|FlowControl|DoOnce false
      (:Completed
        (Audio|PlaySoundatLocation "/Game/Levels/ElectricLevel/drum_stick_hit_sound.drum_stick_hit_sound" (Transformation|GetActorLocation) "0, 0, 0" 1.0 1.0 0.0 0 0 0 0)
        (bind _effectivedamage (CallFunction|GetEffectiveDamage))
        (Game|Damage|ApplyDamage (Variables|Default|GetBoss) _effectivedamage 0 0)
        (CallFunction|Destroy)))))

(fn ConstructionScript)

(fn Deactivate)

(fn SetStartTime
  (Variables|Default|SetStartTime (Actor|GetGameTimeSinceCreation)))

(fn GetEffectiveDamage
  (bind _accuracy (CallFunction|GetAccuracy))
  (return (* (Variables|Default|GetDamage) _accuracy)))

(fn GetAccuracy
  (bind _delay (Variables|Default|GetDelay))
  (return (- 1.0 (/ (Math|Float|Absolute(Float) (- (- (Actor|GetGameTimeSinceCreation) (Variables|Default|GetStartTime)) _delay)) _delay))))

(fn Destroy
  (for _array_element (Variables|Default|Getsiblings)
    (if (and (Utilities|IsValid _array_element) (!= self _array_element))
      (Actor|DestroyActor _array_element)))
  (Actor|DestroyActor))