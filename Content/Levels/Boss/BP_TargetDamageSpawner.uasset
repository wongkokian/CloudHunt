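; Boss-fight spawner that creates damageable targets at random points on a plane and links them to the Boss.
; Points come from nested random lerps between four corner components, retried while they overlap targets in BallSpawned.
; Spawn functions create either electric targets with random blue flag or fire targets, then start them with a delay.
; LookAtPlayer sets yaw along the player-to-spawner direction; the event graph's looping spawn timer is disconnected.
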(event EventBeginPlay)

(event Collision|EventActorBeginOverlap
  (params (OtherActor :type Actor%20Object%20Reference)))

(event EventTick
  (params (DeltaSeconds :type Float%20%28single-precision%29)))

(fn ConstructionScript)

(fn SpawnRBTarget
  (params (Delay :type Float%20%28double-precision%29))
  (while (LocalVariables|GetisColliding)
    (bind _point (CallFunction|GetRandomPointonPlane))
    (bind _output_get (Variables|Default|SetPoint _point))
    (bind _iscolliding (CallFunction|IsCollidingwithOtherCircle _output_get))
    (LocalVariables|SetisColliding _iscolliding))
  (bind _returnvalue (Game|SpawnActorfromClass "/Game/Levels/Boss/ElectricAttack/BP_ElectricDamageable.BP_ElectricDamageable_C" (Math|Transform|MakeTransform (Variables|Default|GetPoint) "0, 0, 0" "1.000000,1.000000,1.000000") "Undefined" 0 0))
  (Variables|/Game/Levels/Boss/ElectricAttack/BP_ElectricDamageable.BP_ElectricDamageable_C|SetBoss _returnvalue (Variables|Default|GetBoss))
  (Default|StartTarget _returnvalue Delay (Math|Random|RandomBool)))

(fn GetRandomPointonPlane
  (LocalVariables|SetPt_A (Transformation|GetWorldLocation (Variables|Default|GetA)))
  (LocalVariables|SetPt_B (Transformation|GetWorldLocation (Variables|Default|GetB)))
  (LocalVariables|SetPt_C (Transformation|GetWorldLocation (Variables|Default|GetC)))
  (LocalVariables|SetPt_D (Transformation|GetWorldLocation (Variables|Default|GetD)))
  (return (Math|Vector|Lerp(Vector) (Math|Vector|Lerp(Vector) (LocalVariables|GetPt_A) (LocalVariables|GetPt_B) (Math|Random|RandomFloat)) (Math|Vector|Lerp(Vector) (LocalVariables|GetPt_C) (LocalVariables|GetPt_D) (Math|Random|RandomFloat)) (Math|Random|RandomFloat))))

(fn IsCollidingwithOtherCircle
  (params (centre :type Vector))
  (bind _result (Utilities|Set|ToArray (Variables|Default|GetBallSpawned)))
  (for _array_element _result
    (if (Utilities|IsValid _array_element)
      (if (<= (Math|Vector|Distance(Vector) centre (Transformation|GetWorldLocation (Variables|/Game/Levels/ElectricLevel/Elec_Rythm_Object/BP_RythmTarget.BP_RythmTarget_C|GetTarget _array_element))) (* (LocalVariables|GetRadius) 2.0))
        (return true))))
  (return false))

(fn LookatPlayer
  (Transformation|SetActorRotation (Math|Rotator|MakeRotator 0.0 0.0 (.yaw (Math|Rotator|FindLookatRotation (Transformation|GetActorLocation (Game|GetPlayerCharacter 0)) (Transformation|GetActorLocation))))))

(fn GetAverageAccuracy
  (bind _average_accuray (|CallParentFunction))
  (return _average_accuray))

(fn UpdateTotalAccuracy
  (params (Accuracy :type Float%20%28double-precision%29) (RythmTarget :type BP%20Rythm%20Target%20Object%20Reference))
  (|CallParentFunction Accuracy RythmTarget))

(fn SpawnTarget
  (params (Delay :type Float%20%28double-precision%29))
  (while (LocalVariables|GetisColliding)
    (bind _point (CallFunction|GetRandomPointonPlane))
    (bind _output_get (Variables|Default|SetPoint _point))
    (bind _iscolliding (CallFunction|IsCollidingwithOtherCircle _output_get))
    (LocalVariables|SetisColliding _iscolliding))
  (bind _returnvalue (Game|SpawnActorfromClass "/Game/Levels/Boss/FireAttack/BP_FireDamageable.BP_FireDamageable_C" (Math|Transform|MakeTransform (Variables|Default|GetPoint) "0, 0, 0" "1.000000,1.000000,1.000000") "Undefined" 0 0))
  (Variables|/Game/Levels/Boss/FireAttack/BP_FireDamageable.BP_FireDamageable_C|SetBoss _returnvalue (Variables|Default|GetBoss))
  (Default|StartTarget _returnvalue Delay))