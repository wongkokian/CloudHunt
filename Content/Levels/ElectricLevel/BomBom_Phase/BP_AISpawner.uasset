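; AI spawner for the BomBom phase of the electric level that spawns randomly red or blue rhythm targets on a plane.
; SpawnBom samples points interpolated between four corner components, using a distance check against spawned targets to avoid overlap.
; While activated, a looping timer sets the spawner's yaw along the player-to-spawner direction; deactivation pauses it.
; Each target references its spawner, whose accuracy functions defer to the parent class.
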(event Custom|Spawn
  (CallFunction|SpawnBom))

(event Custom|End)

(event Custom|Activate%20Spawner
  (Class|KismetSystemLibrary|UnPauseTimer 0 "LookAtPlayer")
  (Utilities|Time|SetTimerbyFunctionName 0 "LookAtPlayer" 0.01 true))

(event Custom|Deactivate%20Spawner
  (Class|KismetSystemLibrary|PauseTimer 0 "LookAtPlayer"))

(event EventBeginPlay)

(event Collision|EventActorBeginOverlap
  (params (OtherActor :type Actor%20Object%20Reference)))

(event EventTick
  (params (DeltaSeconds :type Float%20%28single-precision%29)))

(fn ConstructionScript)

(fn SpawnBom
  (bind _self self)
  (bind _ballspawned (Variables|Default|GetBallSpawned))
  (while (LocalVariables|GetisColliding)
    (bind _point (CallFunction|GetRandomPointonPlane))
    (bind _output_get (Variables|Default|SetPoint _point))
    (Development|PrintString (Utilities|String|ToString(Vector) _output_get))
    (bind _iscolliding (CallFunction|IsCollidingwithOtherCircle _output_get))
    (LocalVariables|SetisColliding _iscolliding))
  (Development|PrintString "Hello")
  (if (Math|Random|RandomBool)
    (bind _returnvalue (Game|SpawnActorfromClass "/Game/Levels/ElectricLevel/Elec_Rythm_Object/BP_RedBlueRythmTarget.BP_RedBlueRythmTarget_C" (Math|Transform|MakeTransform (Variables|Default|GetPoint) "0, 0, 0" "2.500000,2.500000,2.500000") "Undefined" 0 0))
    (Default|StartRedBlueTarget _returnvalue 1.0 false)
    (Variables|/Game/Levels/ElectricLevel/Elec_Rythm_Object/BP_RythmTarget.BP_RythmTarget_C|SetSpawner _returnvalue _self)
    (Utilities|Set|Add _ballspawned _returnvalue)
    (else
      (bind _returnvalue_2 (Game|SpawnActorfromClass "/Game/Levels/ElectricLevel/Elec_Rythm_Object/BP_RedBlueRythmTarget.BP_RedBlueRythmTarget_C" (Math|Transform|MakeTransform (Variables|Default|GetPoint) "0, 0, 0" "2.500000,2.500000,2.500000") "Undefined" 0 0))
      (Default|StartRedBlueTarget _returnvalue_2 1.0 true)
      (Variables|/Game/Levels/ElectricLevel/Elec_Rythm_Object/BP_RythmTarget.BP_RythmTarget_C|SetSpawner _returnvalue_2 _self)
      (Utilities|Set|Add _ballspawned _returnvalue_2))))

(fn GetRandomPointonPlane
  (LocalVariables|SetPt_A (Transformation|GetWorldLocation (Variables|Default|GetA)))
  (LocalVariables|SetPt_B (Transformation|GetWorldLocation (Variables|Default|GetB)))
  (LocalVariables|SetPt_C (Transformation|GetWorldLocation (Variables|Default|GetC)))
  (LocalVariables|SetPt_D (Transformation|GetWorldLocation (Variables|Default|GetD)))
  (return (Math|Vector|Lerp(Vector) (Math|Vector|Lerp(Vector) (LocalVariables|GetPt_A) (LocalVariables|GetPt_B) (Math|Random|RandomFloat)) (Math|Vector|Lerp(Vector) (LocalVariables|GetPt_C) (LocalVariables|GetPt_D) (Math|Random|RandomFloat)) (Math|Random|RandomFloat))))

(fn IsCollidingwithOtherCircle
  (params (centre :type Vector))
  (bind _result (Utilities|Set|ToArray (Variables|Default|GetBallSpawned)))
  (for _array_element _result
    (if (Utilities|IsValid _array_element)
      (if (<= (Math|Vector|Distance(Vector) centre (Transformation|GetWorldLocation (Variables|/Game/Levels/ElectricLevel/Elec_Rythm_Object/BP_RythmTarget.BP_RythmTarget_C|GetTarget _array_element))) (* (LocalVariables|GetRadius) 5.0))
        (return true))))
  (return false))

(fn LookatPlayer
  (Transformation|SetActorRotation (Math|Rotator|MakeRotator 0.0 0.0 (.yaw (Math|Rotator|FindLookatRotation (Transformation|GetActorLocation (Game|GetPlayerCharacter 0)) (Transformation|GetActorLocation))))))

(fn GetAverageAccuracy
  (bind _average_accuray (|CallParentFunction))
  (return _average_accuray))

(fn UpdateTotalAccuracy
  (params (Accuracy :type Float%20%28double-precision%29) (RythmTarget :type BP%20Rythm%20Target%20Object%20Reference))
  (|CallParentFunction Accuracy RythmTarget))