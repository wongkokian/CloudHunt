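; BP_WallBlock is a wall that blows up once it has received all five colors of bomb.
; ReceiveABomb switches on the bomb type and sets a matching boolean record, so order and repeats do not matter.
; When every record is set, it spawns an explosion sound and enlarged particle effect at the mesh, then destroys the actor.
; Debug strings report each received bomb and the completed collection; the event graph is empty.
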(event EventBeginPlay)

(event Collision|EventActorBeginOverlap
  (params (OtherActor :type Actor%20Object%20Reference)))

(event EventTick
  (params (DeltaSeconds :type Float%20%28single-precision%29)))

(fn ConstructionScript)

(fn ReceiveABomb
  (params (BombType :type BombType%20Enum :default "NewEnumerator0"))
  (bind _staticmesh (Variables|Default|GetStaticMesh))
  (bind _returnvalue (Transformation|GetWorldLocation _staticmesh))
  (switch Utilities|FlowControl|Switch|SwitchonBombType BombType
    (:NewEnumerator0
      (Variables|Default|SetRedBombRecord true))
    (:NewEnumerator1
      (Variables|Default|SetBlueBombRecord true))
    (:NewEnumerator2
      (Variables|Default|SetGreenBombRecord true))
    (:NewEnumerator3
      (Variables|Default|SetYelloBombRecord true))
    (:NewEnumerator4
      (Variables|Default|SetWhiteBombRecord true)))
  (if (Math|Boolean|ANDBoolean (Variables|Default|GetRedBombRecord) (Variables|Default|GetBlueBombRecord) (Variables|Default|GetGreenBombRecord) (Variables|Default|GetYelloBombRecord) (Variables|Default|GetWhiteBombRecord))
    (Development|PrintString "collect all kinds of Bomb")
    (Audio|SpawnSoundatLocation "/Game/StarterContent/Audio/Explosion02.Explosion02" _returnvalue "0, 0, 0" 1.0 1.0 0.0 0 0)
    (Effects|SpawnEmitteratLocation "/Game/StarterContentMin/Particles/P_Explosion.P_Explosion" _returnvalue "0, 0, 0" "4.000000,4.000000,4.000000")
    (Actor|DestroyActor)
    (else
      (Development|PrintString "received a Bomb"))))