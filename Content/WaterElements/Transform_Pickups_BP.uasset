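; Water-level pickup actor tied to one of three sea-creature forms (shark, tuna or manta ray) through a target index.
; The construction script sets the skeletal mesh from that index.
; When a Fish overlaps the interact collision, its transform index is compared to the target and a success or fail message prints.
; Either result increments the score on WaterLevelInstance actors found in the level and destroys the pickup.
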(event OnComponentBeginOverlap(Sphere)
  (params (OverlappedComponent :type Primitive%20Component%20Object%20Reference) (OtherActor :type Actor%20Object%20Reference) (OtherComp :type Primitive%20Component%20Object%20Reference) (OtherBodyIndex :type Integer) (bFromSweep :type Boolean) (SweepResult :type Hit%20Result%20Structure%20%28by%20ref%29)))

(event OnComponentBeginOverlap(InteractCollision)
  (params (OverlappedComponent :type Primitive%20Component%20Object%20Reference) (OtherActor :type Actor%20Object%20Reference) (OtherComp :type Primitive%20Component%20Object%20Reference) (OtherBodyIndex :type Integer) (bFromSweep :type Boolean) (SweepResult :type Hit%20Result%20Structure%20%28by%20ref%29))
  (bind _asfish (Utilities|Casting|CastToFish OtherActor))
  (if (== (Variables|/Game/WaterElements/Fish.Fish_C|GetTransformIndex _asfish) (Variables|Default|GetTargetIndex))
    (Development|PrintString "Success")
    (Development|PrintString "+ 1")
    (else
      (Development|PrintString "Fail")))
  (bind _outactors (Actor|GetAllActorsOfClass "/Game/WaterElements/WaterLevelInstance.WaterLevelInstance_C"))
  (Default|IncrementScore _outactors)
  (Actor|DestroyActor))

(event OnComponentEndOverlap(InteractCollision)
  (params (OverlappedComponent :type Primitive%20Component%20Object%20Reference) (OtherActor :type Actor%20Object%20Reference) (OtherComp :type Primitive%20Component%20Object%20Reference) (OtherBodyIndex :type Integer)))

(event Input|ActionEvents|InputActioninteract
  (params (Key :type Key%20Structure :default "None")))

(fn ConstructionScript
  (bind _skeletalmesh (Variables|Default|GetSkeletalMesh))
  (switch int (Variables|Default|GetTargetIndex)
    (:0
      (Class|SkinnedMeshComponent|SetSkeletalMesh _skeletalmesh "/Game/WaterElements/great-white-shark/source/shark.shark" true))
    (:1
      (Class|SkinnedMeshComponent|SetSkeletalMesh _skeletalmesh "/Game/WaterElements/tuna-fish/source/TunaFish.TunaFish" true))
    (:2
      (Class|SkinnedMeshComponent|SetSkeletalMesh _skeletalmesh "/Game/WaterElements/model-84b-manta-ray-swimming/source/manta-ray_animation_08.manta-ray_animation_08" true))))