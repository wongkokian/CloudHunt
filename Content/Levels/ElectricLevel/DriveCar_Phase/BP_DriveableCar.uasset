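; Possessable car for the electric level's driving phase that rides the CarTrack spline on rails.
; A timeline drives position and rotation along the spline, while A and D shift the mesh between three lanes.
; Left click box-traces ahead for a BP_DriveableTarget, then spawns a BP_Trace fed sampled spline transforms between both alphas and the current lane.
; M returns possession and camera to the player character and hides the car.
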(event Custom|Move%20Car
  (bind _carmover (Variables|Default|GetCarMover))
  (bind _cartrack (Variables|Default|GetCarTrack))
  (bind _spline (Variables|/Game/Levels/ElectricLevel/Elec_Phases/Car_Phase/CarTrackNew.CarTrackNew_C|GetSpline _cartrack))
  (Components|Timeline|SetPlayRate _carmover (/ 1.0 (Variables|Default|GetDuration)))
  (Components|Timeline|SetNewTime _carmover (Variables|Default|GetCar%20Start%20Offset))
  (bind _alpha (Timeline|CarMover Play)
    (:Update
      (Variables|Default|SetAlpha _alpha)
      (Transformation|SetActorLocationAndRotation (Spline|GetLocationatDistanceAlongSpline _spline (Math|Float|Lerp 0.0 (Spline|GetSplineLength _spline) (Variables|Default|GetAlpha)) "World") (Spline|GetRotationatDistanceAlongSpline _spline (Math|Float|Lerp 0.0 (Spline|GetSplineLength _spline) (Variables|Default|GetAlpha)) "World")))))

(event Custom|CameraOverride
  (Variables|Default|SetbFindCameraComponentWhenViewTarget true)
  (Game|Player|SetViewTargetwithBlend (Game|GetPlayerController 0) (Components|GetOwner (Variables|Default|GetCamera)) 0.0 "VTBlend_Linear" 0.0 false))

(event Custom|DeleteCar
  (Actor|DestroyActor))

(event Custom|Possess%20Car
  (Pawn|Possess (Game|GetPlayerController 0) self)
  (CallFunction|CameraOverride)
  (CallFunction|MoveCar))

(event EventBeginPlay)

(event Input|KeyboardEvents|D
  (params (Key :type Key%20Structure :default "None"))
  (:Pressed
    (if (!= (Variables|Default|GetPositionState) 2)
      (Transformation|AddLocalOffset (Variables|Default|GetCarMesh) "0,500.000000, 0" false false)
      (Math|Integer|IncrementInt (Variables|Default|GetPositionState)))))

(event Input|KeyboardEvents|A
  (params (Key :type Key%20Structure :default "None"))
  (:Pressed
    (if (!= (Variables|Default|GetPositionState) 0)
      (Transformation|AddLocalOffset (Variables|Default|GetCarMesh) "0,-500.000000, 0" false false)
      (Math|Integer|DecrementInt (Variables|Default|GetPositionState)))))

(event Input|KeyboardEvents|M
  (params (Key :type Key%20Structure :default "None"))
  (bind _returnvalue (Game|GetPlayerController 0))
  (bind _playercharacterref (Variables|Default|GetPlayerCharacterRef))
  (bind _als_cameramanager (Variables|/Game/AdvancedLocomotionV4/Blueprints/CharacterLogic/ALS_AnimMan_CharacterBP.ALS_AnimMan_CharacterBP_C|GetALS_CameraManager _playercharacterref))
  (:Pressed
    (Pawn|Possess _returnvalue _playercharacterref)
    (Variables|/Script/Engine.Actor|SetbFindCameraComponentWhenViewTarget _als_cameramanager true)
    (Game|Player|SetViewTargetwithBlend _returnvalue (Components|GetOwner (Variables|/Game/AdvancedLocomotionV4/Blueprints/CameraSystem/ALS_PlayerCameraManager.ALS_PlayerCameraManager_C|GetCameraBehavior _als_cameramanager)) 0.0 "VTBlend_Linear" 0.0 false)
    (Rendering|SetActorHiddenInGame true)))

(event Input|MouseEvents|LeftMouseButton
  (params (Key :type Key%20Structure :default "None"))
  (bind _carmesh (Variables|Default|GetCarMesh))
  (bind _returnvalue (Transformation|GetWorldLocation _carmesh))
  (:Pressed
    (bind _outhit (Collision|BoxTraceByChannel _returnvalue (+ _returnvalue (* (Math|Vector|GetForwardVector _carmesh) "1500.000000,1500.000000,1500.000000")) "50.000000,50.000000,50.000000" (Transformation|GetWorldRotation _carmesh) "TraceTypeQuery3" false 0 "ForDuration"))
    (bind _asbp_driveable_target (Utilities|Casting|CastToBP_DriveableTarget (.hitactor _outhit)))
    (bind _positions (CallFunction|InterpolateSpline (Variables|Default|GetAlpha) (Variables|/Game/Levels/ElectricLevel/BP_DriveableTarget.BP_DriveableTarget_C|GetAlpha _asbp_driveable_target) 20))
    (bind _returnvalue_2 (Game|SpawnActorfromClass "/Game/Levels/ElectricLevel/BP_Trace.BP_Trace_C" (Transformation|GetWorldTransform (Variables|Default|GetCarMesh)) "Undefined" 0 0))
    (Default|Init _returnvalue_2 _positions 20 0.1 (Variables|Default|GetPositionState))
    (Default|Start _returnvalue_2)))

(fn ConstructionScript)

(fn LocationatSplineatTime
  (params (Time :type Float%20%28double-precision%29))
  (bind _cartrack (Variables|Default|GetCarTrack))
  (bind _spline (Variables|/Game/Levels/ElectricLevel/Elec_Phases/Car_Phase/CarTrackNew.CarTrackNew_C|GetSpline _cartrack))
  (LocalVariables|SetTimeAlpha (/ Time (Variables|Default|GetDuration)))
  (return (Math|Transform|MakeTransform (Spline|GetLocationatDistanceAlongSpline _spline (Math|Float|Lerp 0.0 (Spline|GetSplineLength _spline) (LocalVariables|GetTimeAlpha)) "World") (Spline|GetRotationatDistanceAlongSpline _spline (Math|Float|Lerp 0.0 (Spline|GetSplineLength _spline) (LocalVariables|GetTimeAlpha)) "World") "1.000000,1.000000,1.000000")))

(fn GetCameraLocation
  (return (Transformation|GetWorldLocation (Variables|Default|GetCamera))))

(fn InterpolateSpline
  (params (StartAlpha :type Float%20%28double-precision%29) (EndAlpha :type Float%20%28double-precision%29) (SampleRate :type Integer))
  (for _index (range 0 SampleRate)
    (bind _transform (CallFunction|LocationatSplineatAlpha (Math|Float|Lerp StartAlpha EndAlpha (/ (Math|Conversions|ToFloat(Integer) _index) (Math|Conversions|ToFloat(Integer) SampleRate)))))
    (Utilities|Array|Add (LocalVariables|GetOutputs) _transform))
  (return (LocalVariables|GetOutputs)))

(fn LocationatSplineatAlpha
  (params (Alpha :type Float%20%28double-precision%29))
  (bind _cartrack (Variables|Default|GetCarTrack))
  (bind _spline (Variables|/Game/Levels/ElectricLevel/Elec_Phases/Car_Phase/CarTrackNew.CarTrackNew_C|GetSpline _cartrack))
  (bind _returnvalue (Spline|GetSplineLength _spline))
  (bind _returnvalue_2 (Math|Float|Lerp 0.0 _returnvalue Alpha))
  (return (Math|Transform|MakeTransform (Spline|GetLocationatDistanceAlongSpline _spline _returnvalue_2 "World") (Spline|GetRotationatDistanceAlongSpline _spline _returnvalue_2 "World") "1.000000,1.000000,1.000000")))