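; Controller for the second Red Blue phase of the electric level, extending a parent phase controller with start, reset, completion and accuracy handling.
; Sequencer events step through beat times to make the Robot's spawner spawn red/blue targets, and later complete the phase.
; Starting the phase retunes player movement, and the player overlapping the End volume flags completion.
; Resets clear balls and re-enable End collision; the Range-exit handler is empty, leaving its reset logic unreachable.
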(event OnComponentEndOverlap(Range)
  (params (OverlappedComponent :type Primitive%20Component%20Object%20Reference) (OtherActor :type Actor%20Object%20Reference) (OtherComp :type Primitive%20Component%20Object%20Reference) (OtherBodyIndex :type Integer)))

(event OnComponentBeginOverlap(End)
  (params (OverlappedComponent :type Primitive%20Component%20Object%20Reference) (OtherActor :type Actor%20Object%20Reference) (OtherComp :type Primitive%20Component%20Object%20Reference) (OtherBodyIndex :type Integer) (bFromSweep :type Boolean) (SweepResult :type Hit%20Result%20Structure%20%28by%20ref%29))
  (Development|PrintString "ENDDD 
")
  (if (== (Utilities|GetClass OtherActor) "/Game/AdvancedLocomotionV4/Blueprints/CharacterLogic/ALS_Player.ALS_Player_C")
    (Utilities|FlowControl|DoOnce false :!label _label
      (:Completed
        (Variables|Default|SetisComplete true)
        (goto _label Reset)))))

(event EventBeginPlay
  (CallFunction|Init))

(event Custom|Spawn%20Target
  (bind _beatcounter (Variables|Default|GetBeatCounter))
  (Default|SpawnRedBlue (Variables|Default|GetSpawner) (Utilities|Array|Get(acopy) (Variables|Default|GetBeatTime) _beatcounter))
  (Math|Integer|IncrementInt _beatcounter))

(event Custom|Complete%20Red%20Blue%202
  (CallFunction|Complete))

(fn ConstructionScript)

(fn TriggerPhase
  (Development|PrintString "Red Blue\\ 2")
  (Variables|Default|SetHasStarted true)
  (|CallParentFunction)
  (Default|SetPlayerMovement (Variables|Default|GetElectricLevelController) 2.25e+03 5.0))

(fn ResetPhase
  (Default|RemoveAllBalls (Variables|Default|GetSpawner))
  (Variables|Default|SetBeatCounter 0)
  (CallFunction|EnableCollision)
  (|CallParentFunction))

(fn Init
  (Variables|Default|SetEndTransform (Transformation|GetRelativeTransform (Variables|Default|GetEnd)))
  (Variables|Default|SetRangeTransform (Transformation|GetRelativeTransform (Variables|Default|GetRange)))
  (bind _asbp_red_blue_2spawner (Default|GetRedBlue2Spawner (Variables|Default|GetRobot)))
  (bind _output_get (Variables|Default|SetSpawner _asbp_red_blue_2spawner))
  (Variables|/Game/Levels/ElectricLevel/Spawner/BP_Spawner.BP_Spawner_C|SetPhaseController _output_get self)
  (|CallParentFunction))

(fn GetAccuracy
  (bind _average_accuray (Default|GetAverageAccuracy (Variables|Default|GetSpawner)))
  (return _average_accuray))

(fn EndPhase
  (|CallParentFunction)
  (Default|ResetAccuracy (Variables|Default|GetSpawner)))

(fn EnableCollision
  (Collision|SetCollisionEnabled (Variables|Default|GetEnd) "QueryOnly"))

(fn DisableCollision
  (Collision|SetCollisionEnabled (Variables|Default|GetEnd) "NoCollision"))

(fn ActivateController
  (CallFunction|ResetPhase)
  (|CallParentFunction))

(fn DeactivateController
  (CallFunction|DisableCollision)
  (|CallParentFunction))