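; BP_testMoving is a test actor in the WeatherSystem folder that moves a cube along a spline in a continuous loop.
; Each Tick advances a distance by Speed times DeltaSeconds and samples the spline's local transform there.
; The cube takes that location and rotation as its relative transform, keeping its own scale.
; The distance resets to zero once it passes the spline's length.
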(event EventBeginPlay)

(event Collision|EventActorBeginOverlap
  (params (OtherActor :type Actor%20Object%20Reference)))

(event EventTick
  (params (DeltaSeconds :type Float%20%28single-precision%29))
  (Variables|Default|Setdistance (+ (* DeltaSeconds (Variables|Default|Getspeed)) (Variables|Default|Getdistance)))
  (Transformation|SetRelativeTransform (Variables|Default|GetCube) (Math|Transform|MakeTransform (.location (Spline|GetTransformatDistanceAlongSpline (Variables|Default|GetSpline) (Variables|Default|Getdistance) "Local" false)) (.rotation (Spline|GetTransformatDistanceAlongSpline (Variables|Default|GetSpline) (Variables|Default|Getdistance) "Local" false)) (Variables|/Script/Engine.SceneComponent|GetRelativeScale3D (Variables|Default|GetCube))) false false)
  (if (> (Variables|Default|Getdistance) (Spline|GetSplineLength (Variables|Default|GetSpline)))
    (Variables|Default|Setdistance 0.0)))

(fn ConstructionScript)