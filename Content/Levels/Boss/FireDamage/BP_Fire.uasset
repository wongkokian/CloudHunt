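; BP_Fire is a short-lived fire actor in the boss level's FireDamage folder.
; It destroys itself after a Duration delay from BeginPlay.
; The first overlap with any actor only prints "Hit Player" through a DoOnce, with no damage applied.
; GetLength returns the world-space distance between its Start and End components.
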(event EventBeginPlay
  (Utilities|FlowControl|Delay (Variables|Default|Getduration))
  (Actor|DestroyActor))

(event Collision|EventActorBeginOverlap
  (params (OtherActor :type Actor%20Object%20Reference))
  (Utilities|FlowControl|DoOnce false
    (:Completed
      (Development|PrintString "Hit Player"))))

(event EventTick
  (params (DeltaSeconds :type Float%20%28single-precision%29)))

(fn ConstructionScript)

(fn GetLength
  (return (Math|Vector|Distance(Vector) (Transformation|GetWorldLocation (Variables|Default|GetStart)) (Transformation|GetWorldLocation (Variables|Default|GetEnd)))))