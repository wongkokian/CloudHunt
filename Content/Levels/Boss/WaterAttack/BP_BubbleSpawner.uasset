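; BP_BubbleSpawner is a boss water-attack actor that spawns rings of damageable bubbles around a center point.
; On BeginPlay it precomputes evenly spaced angles, measures the radius from Center to End and starts a looping timer.
; Each tick of that timer places bubbles on a circle scaled by a countdown from the Delays count, so rings close inward.
; Each bubble receives the Boss reference and is started; spawning stops once the countdown drops below zero.
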(event EventBeginPlay
  (CallFunction|Init 5 (Variables|Default|Getd))
  (Variables|Default|Setradius (Math|Vector|Distance(Vector) (Transformation|GetWorldLocation (Variables|Default|Getcenter)) (Transformation|GetWorldLocation (Variables|Default|Getend))))
  (Variables|Default|Setc (Transformation|GetWorldLocation (Variables|Default|Getcenter)))
  (Utilities|Time|SetTimerbyFunctionName 0 "SpawnBubblesRing" 2.0 true))

(event Collision|EventActorBeginOverlap
  (params (OtherActor :type Actor%20Object%20Reference)))

(event EventTick
  (params (DeltaSeconds :type Float%20%28single-precision%29)))

(fn ConstructionScript)

(fn Init
  (params (Theta :type Integer) (Delays :type Array%20of%20Floats%20%28double-precision%29))
  (Variables|Default|SetTheta Theta)
  (bind _output_get (Variables|Default|SetDelays Delays))
  (Variables|Default|SetCounter (Utilities|Array|Length _output_get))
  (for _index (range 1 (Variables|Default|GetTheta))
    (Utilities|Array|Add (LocalVariables|Geta) (* (Math|Float|MultiplybyPi 2.0) (/ _index (Variables|Default|GetTheta)))))
  (Variables|Default|Setangles (LocalVariables|Geta)))

(fn GetPointsonCircle
  (bind _delays (Variables|Default|GetDelays))
  (bind _c (Variables|Default|Getc))
  (bind _returnvalue (Utilities|Array|Length _delays))
  (LocalVariables|SetNumParts (+ _returnvalue (/ _returnvalue 4)))
  (for _array_element (Variables|Default|Getangles)
    (Utilities|Array|Add (LocalVariables|GetLocations) (Math|Vector|MakeVector (+ (* (Math|Trig|Cos(Radians) _array_element) (* (Variables|Default|Getradius) (/ (Variables|Default|GetCounter) (LocalVariables|GetNumParts)))) (.x _c)) (+ (* (Math|Trig|Sin(Radians) _array_element) (* (Variables|Default|Getradius) (/ (Variables|Default|GetCounter) (LocalVariables|GetNumParts)))) (.y _c)) (.z _c))))
  (return (LocalVariables|GetLocations)))

(fn SpawnBubblesRing
  (Development|PrintString "Hello")
  (if (>= (Variables|Default|GetCounter) 0)
    (bind _location (CallFunction|GetPointsonCircle))
    (for _array_element _location
      (bind _returnvalue (Game|SpawnActorfromClass "/Game/Levels/Boss/WaterAttack/BP_BubbleDamageable.BP_BubbleDamageable_C" (Math|Transform|MakeTransform _array_element "0, 0, 0" "1.000000,1.000000,1.000000") "Undefined" 0 0))
      (if (Utilities|IsValid _returnvalue)
        (Variables|/Game/Levels/Boss/WaterAttack/BP_BubbleDamageable.BP_BubbleDamageable_C|SetBoss _returnvalue (Variables|Default|GetBoss))
        (Default|StartBubble _returnvalue 1.0)))
    (Math|Integer|DecrementInt (Variables|Default|GetCounter))))