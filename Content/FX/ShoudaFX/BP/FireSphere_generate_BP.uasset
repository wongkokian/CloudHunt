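; Trigger actor in the Shouda FX set that spawns fire spheres when another actor overlaps it.
; On ActorBeginOverlap it spawns a FireSphere at the world transform of each of four point components.
; It does not filter the overlapping actor or guard against re-triggering, so every new overlap spawns another full set.
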(event Collision|EventActorBeginOverlap
  (params (OtherActor :type Actor%20Object%20Reference))
  (Game|SpawnActorfromClass "/Game/FX/ShoudaFX/BP/FireSphere.FireSphere_C" (Transformation|GetWorldTransform (Variables|Default|GetPOINT2)) "Undefined" 0 0)
  (Game|SpawnActorfromClass "/Game/FX/ShoudaFX/BP/FireSphere.FireSphere_C" (Transformation|GetWorldTransform (Variables|Default|GetPOINT1)) "Undefined" 0 0)
  (Game|SpawnActorfromClass "/Game/FX/ShoudaFX/BP/FireSphere.FireSphere_C" (Transformation|GetWorldTransform (Variables|Default|GetPOINT)) "Undefined" 0 0)
  (Game|SpawnActorfromClass "/Game/FX/ShoudaFX/BP/FireSphere.FireSphere_C" (Transformation|GetWorldTransform (Variables|Default|GetPOINT3)) "Undefined" 0 0))

(fn ConstructionScript)