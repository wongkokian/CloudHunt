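; Interactable NPC that steps through an array of dialogue messages on the HUD, one per interaction.
; Each interaction briefly hides then redraws the dialogue via a HUD actor found on BeginPlay, closing it after the last line.
; Ending overlap hides the dialogue and resets progress.
; Highlighting uses custom depth, with stencil color mapped from Level, and a DoOnce clears it upon interaction until overlap ends.
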(event Custom|Show%20Dialouge
  (CallFunction|HideDialouge)
  (Utilities|FlowControl|Delay 0.1)
  (CallFunction|DisplayDialouge))

(event EventBeginPlay
  (CallFunction|SetColor)
  (bind _outactors (Actor|GetAllActorsOfClass "/Game/UI/HUDActor.HUDActor_C"))
  (Variables|Default|SetHudActor (Utilities|Array|Get(acopy) _outactors)))

(event Collision|EventActorBeginOverlap
  (params (OtherActor :type Actor%20Object%20Reference)))

(event EventTick
  (params (DeltaSeconds :type Float%20%28single-precision%29)))

(event EventInteract
  (|CallParentFunction)
  (CallFunction|ShowDialouge)
  (Utilities|FlowControl|DoOnce false
    (:Completed
      (CallFunction|UntoggleHighlight))))

(event Collision|EventActorEndOverlap
  (params (OtherActor :type Actor%20Object%20Reference))
  (|CallParentFunction 0)
  (CallFunction|HideDialouge)
  (Variables|Default|SetHasEnded false)
  (Variables|Default|Setcounter 0)
  (Utilities|FlowControl|DoOnce false) ; enters at Reset
)

(fn ConstructionScript)

(fn DoStuff)

(fn ToggleHighlight
  (Rendering|SetRenderCustomDepth (Variables|Default|GetSkeletalMesh) true)
  (|CallParentFunction))

(fn UntoggleHighlight
  (Rendering|SetRenderCustomDepth (Variables|Default|GetSkeletalMesh) false)
  (|CallParentFunction))

(fn DisplayDialouge
  (Development|PrintString (Utilities|String|ToString(Integer) (Variables|Default|Getcounter)))
  (if (Variables|Default|GetHasEnded)
    (CallFunction|HideDialouge)
    (Variables|Default|Setcounter 0)
    (Variables|Default|SetHasEnded false)
    (else
      (bind _hudref (Default|GetHudRef (Variables|Default|GetHudActor)))
      (Default|DisplayDialogue _hudref (Utilities|Array|Get(acopy) (Variables|Default|Getmessages) (Variables|Default|Getcounter)) (Variables|Default|GetName))
      (bind _result (Math|Integer|IncrementInt (Variables|Default|Getcounter))
        (:%20%20
          (if (== _result (Utilities|Array|Length (Variables|Default|Getmessages)))
            (Variables|Default|SetHasEnded true)))))))

(fn SetColor
  (Rendering|SetCustomDepthStencilValue (Variables|Default|GetSkeletalMesh) (.Value (Utilities|Map|Find (Variables|Default|GetColorMapping) (Variables|Default|Getlevel)))))

(fn HideDialouge
  (bind _hudref (Default|GetHudRef (Variables|Default|GetHudActor)))
  (Default|HideDialogue _hudref))

(fn SetMessages
  (params (Messages :type Array%20of%20Strings))
  (Variables|Default|Setmessages Messages))