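; BP_AI_Controller runs the AI robot phase of the electric level, extending a parent phase class.
; TriggerPhase activates the spawner, reveals the robot, teleports the player to the start and plays a Level Sequence whose events drive spawning and phase end.
; EndPhase reports the spawner's average accuracy to the level controller, moves the player out and resets the spawner.
; Timelines animate an outline radius through a material parameter collection centred on the player.
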(event Custom|Add%20Outline%20Post%20Process
  (Rendering|Material|SetVectorParameterValue "/Game/Materials/PC_Outline.PC_Outline" "Position" (Math|Conversions|ToLinearColor(Vector) (Transformation|GetWorldLocation (Variables|/Script/Engine.Actor|GetRootComponent (Game|GetPlayerCharacter 0)))) :!class /Script/Engine.KismetMaterialLibrary)
  (bind _newtrack_0 (Timeline|Timeline_0 Play)
    (:Update
      (Rendering|Material|SetScalarParameterValue "/Game/Materials/PC_Outline.PC_Outline" "Radius" _newtrack_0 :!class /Script/Engine.KismetMaterialLibrary))))

(event Custom|Remove%20Outline%20Post%20Process
  (Rendering|Material|SetVectorParameterValue "/Game/Materials/PC_Outline.PC_Outline" "Position" (Math|Conversions|ToLinearColor(Vector) (Transformation|GetWorldLocation (Variables|/Script/Engine.Actor|GetRootComponent (Game|GetPlayerCharacter 0)))) :!class /Script/Engine.KismetMaterialLibrary)
  (bind _newtrack_0 (Timeline|Timeline_1 Play)
    (:Update
      (Rendering|Material|SetScalarParameterValue "/Game/Materials/PC_Outline.PC_Outline" "Radius" _newtrack_0 :!class /Script/Engine.KismetMaterialLibrary))))

(event EventBeginPlay
  (CallFunction|Init))

(event Collision|EventActorBeginOverlap
  (params (OtherActor :type Actor%20Object%20Reference)))

(event EventTick
  (params (DeltaSeconds :type Float%20%28single-precision%29)))

(event Custom|End%20Spawner)

(event Custom|End
  (params (Owner :type Actor%20Object%20Reference))
  (CallFunction|EndPhase))

(event Custom|Spawn
  (params (Owner :type Actor%20Object%20Reference))
  (CallFunction|SpawnObject))

(event Custom|SequenceEvent_0
  (Variables|Default|SetisComplete true)
  (CallFunction|Complete))

(fn ConstructionScript)

(fn Respawn)

(fn TriggerPhase
  (Default|ActivateSpawner (Variables|Default|GetSpawner))
  (Rendering|SetActorHiddenInGame (Variables|Default|GetSpawner) false)
  (Rendering|SetActorHiddenInGame (Variables|Default|GetAIRobot) false)
  (Transformation|SetActorLocation (Game|GetPlayerCharacter 0) (Transformation|GetWorldLocation (Variables|Default|GetStartLocation)) false true)
  (bind _outactor (Sequencer|Player|CreateLevelSequencePlayer "/Game/Levels/ElectricLevel/AIRobotSeq.AIRobotSeq"))
  (Sequencer|Player|Play (Variables|/Script/LevelSequence.LevelSequenceActor|GetSequencePlayer _outactor) :!class /Script/MovieScene.MovieSceneSequencePlayer)
  (Default|ResetPlayerMovement (Variables|Default|GetElectricLevelController))
  (CallFunction|AddOutlinePostProcess)
  (|CallParentFunction))

(fn FixPlayerLocation
  (Transformation|SetActorLocation (Transformation|GetWorldLocation (Variables|Default|GetStartLocation)) false true))

(fn SpawnObject
  (Default|Spawn (Variables|Default|GetSpawner)))

(fn EnableCollision)

(fn DisableCollision)

(fn EndPhase
  (bind _spawner (Variables|Default|GetSpawner))
  (CallFunction|RemoveOutlinePostProcess)
  (Rendering|SetActorHiddenInGame (Variables|Default|GetAIRobot) true)
  (bind _average_accuray (Default|GetAverageAccuracy (Variables|Default|GetSpawner)))
  (Default|CompletePhase (Variables|Default|GetElectricLevelController) _average_accuray)
  (Transformation|SetActorLocation (Game|GetPlayerCharacter 0) (Transformation|GetWorldLocation (Variables|Default|GetEndLocation)) false true)
  (Pawn|SetControlRotation (Game|GetPlayerController 0) (Transformation|GetWorldRotation (Variables|Default|GetEndLocation)))
  (Rendering|SetActorHiddenInGame (Variables|Default|GetSpawner) true)
  (Default|ResetAccuracy _spawner)
  (Default|DeactivateSpawner _spawner)
  (|CallParentFunction))

(fn GetAccuracy
  (bind _average_accuray (Default|GetAverageAccuracy (Variables|Default|GetSpawner)))
  (return _average_accuray))

(fn Init
  (Variables|/Game/Levels/ElectricLevel/Spawner/BP_Spawner.BP_Spawner_C|SetPhaseController (Variables|Default|GetSpawner) self)
  (|CallParentFunction))