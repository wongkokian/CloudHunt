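; Ambience controller actor that switches looping background sound between forest, sea and volcano as overlaps begin or end on region components, starting with sea.
; Entering the sea or volcano region selects that ambience, and leaving either returns to forest.
; A second Overlap audio component plays the outgoing sound with a long fade-out to mask each switch.
; The main Ambience component fades between sounds, but the volcano switch skips the delay after fade-out.
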(event OnComponentBeginOverlap(SeaRegion)
  (params (OverlappedComponent :type Primitive%20Component%20Object%20Reference) (OtherActor :type Actor%20Object%20Reference) (OtherComp :type Primitive%20Component%20Object%20Reference) (OtherBodyIndex :type Integer) (bFromSweep :type Boolean) (SweepResult :type Hit%20Result%20Structure%20%28by%20ref%29))
  (CallFunction|OverlapSound "/Game/AmbienceMusice/forest_ambience.forest_ambience")
  (CallFunction|SetSeaAmbiance))

(event OnComponentEndOverlap(SeaRegion)
  (params (OverlappedComponent :type Primitive%20Component%20Object%20Reference) (OtherActor :type Actor%20Object%20Reference) (OtherComp :type Primitive%20Component%20Object%20Reference) (OtherBodyIndex :type Integer))
  (CallFunction|OverlapSound "/Game/AmbienceMusice/sea_ambience.sea_ambience")
  (CallFunction|SetForestAmbience))

(event OnComponentBeginOverlap(VolcanoRegion)
  (params (OverlappedComponent :type Primitive%20Component%20Object%20Reference) (OtherActor :type Actor%20Object%20Reference) (OtherComp :type Primitive%20Component%20Object%20Reference) (OtherBodyIndex :type Integer) (bFromSweep :type Boolean) (SweepResult :type Hit%20Result%20Structure%20%28by%20ref%29))
  (CallFunction|OverlapSound "/Game/AmbienceMusice/forest_ambience.forest_ambience")
  (CallFunction|SetVolcanoAmbiance))

(event OnComponentEndOverlap(VolcanoRegion)
  (params (OverlappedComponent :type Primitive%20Component%20Object%20Reference) (OtherActor :type Actor%20Object%20Reference) (OtherComp :type Primitive%20Component%20Object%20Reference) (OtherBodyIndex :type Integer))
  (CallFunction|OverlapSound "/Game/AmbienceMusice/volcano_ambience.volcano_ambience")
  (CallFunction|SetForestAmbience))

(event Custom|OverlapSound
  (params (sound :type Sound%20Base%20Object%20Reference))
  (bind _overlap (Variables|Default|GetOverlap))
  (Audio|Components|Audio|SetSound _overlap sound)
  (Audio|Components|Audio|Play _overlap 0.0)
  (Audio|Components|Audio|FadeOut _overlap 5.0 0.0 "Linear" :!class /Script/Engine.AudioComponent))

(event Custom|wait
  (Utilities|FlowControl|Delay 1.0))

(event Custom|Set%20Forest%20Ambience
  (bind _ambience (Variables|Default|Getambience))
  (Audio|Components|Audio|FadeOut _ambience 1.0 0.0 "Linear" :!class /Script/Engine.AudioComponent)
  (Utilities|FlowControl|Delay 1.0)
  (Audio|Components|Audio|SetSound _ambience "/Game/AmbienceMusice/forest_ambience.forest_ambience")
  (Audio|Components|Audio|Play _ambience 0.0)
  (Audio|Components|Audio|FadeIn _ambience 1.0 1.0 0.0 "Linear" :!class /Script/Engine.AudioComponent))

(event Custom|Set%20Sea%20Ambiance
  (bind _ambience (Variables|Default|Getambience))
  (Audio|Components|Audio|FadeOut _ambience 1.0 0.0 "Linear" :!class /Script/Engine.AudioComponent)
  (Utilities|FlowControl|Delay 1.0)
  (Audio|Components|Audio|SetSound _ambience "/Game/AmbienceMusice/sea_ambience.sea_ambience")
  (Audio|Components|Audio|Play _ambience 0.0)
  (Audio|Components|Audio|FadeIn _ambience 1.0 1.0 0.0 "Linear" :!class /Script/Engine.AudioComponent))

(event Custom|Set%20Volcano%20Ambiance
  (bind _ambience (Variables|Default|Getambience))
  (Audio|Components|Audio|FadeOut _ambience 1.0 0.0 "Linear" :!class /Script/Engine.AudioComponent)
  (Audio|Components|Audio|SetSound _ambience "/Game/AmbienceMusice/volcano_ambience.volcano_ambience")
  (Audio|Components|Audio|Play _ambience 0.0)
  (Audio|Components|Audio|FadeIn _ambience 1.0 1.0 0.0 "Linear" :!class /Script/Engine.AudioComponent))

(event EventBeginPlay
  (CallFunction|SetSeaAmbiance))

(event Collision|EventActorBeginOverlap
  (params (OtherActor :type Actor%20Object%20Reference)))

(event EventTick
  (params (DeltaSeconds :type Float%20%28single-precision%29)))

(fn ConstructionScript)