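; Jet stream water element that switches the player into a Fish pawn and propels it with trigger volumes.
; Transform overlap teleports the ALS_Player to the world origin, then possesses the level's Fish, zeroes its velocity and moves it to StartLocation.
; Plane overlap launches a Fish along the plane's up vector with a velocity-change impulse.
; Leaving Entercurve calls MoveInJetstream on the Fish, found by class lookup regardless of what overlapped.
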(event OnComponentBeginOverlap(Plane)
  (params (OverlappedComponent :type Primitive%20Component%20Object%20Reference) (OtherActor :type Actor%20Object%20Reference) (OtherComp :type Primitive%20Component%20Object%20Reference) (OtherBodyIndex :type Integer) (bFromSweep :type Boolean) (SweepResult :type Hit%20Result%20Structure%20%28by%20ref%29))
  (bind _plane (Variables|Default|GetPlane))
  (bind _returnvalue (Math|Vector|GetUpVector _plane))
  (bind _returnvalue_2 (* _returnvalue "1000.000000,1000.000000,1000.000000"))
  (bind _asfish (Utilities|Casting|CastToFish OtherActor))
  (Physics|AddImpulse (Variables|/Script/Engine.DefaultPawn|GetCollisionComponent _asfish) _returnvalue_2 "None" true)
  (Development|PrintString (Utilities|String|ToString(Vector) _returnvalue_2)))

(event OnComponentBeginOverlap(transform)
  (params (OverlappedComponent :type Primitive%20Component%20Object%20Reference) (OtherActor :type Actor%20Object%20Reference) (OtherComp :type Primitive%20Component%20Object%20Reference) (OtherBodyIndex :type Integer) (bFromSweep :type Boolean) (SweepResult :type Hit%20Result%20Structure%20%28by%20ref%29))
  (bind _asals_player (Utilities|Casting|CastToALS_Player OtherActor))
  (bind _returnvalue (Actor|GetActorOfClass "/Game/WaterElements/Fish.Fish_C"))
  (Transformation|Teleport _asals_player "0, 0, 0" "0, 0, 0")
  (Class|PrimitiveComponent|SetAllPhysicsLinearVelocity (Variables|/Script/Engine.DefaultPawn|GetMeshComponent _returnvalue) "0, 0, 0" false)
  (Development|PrintString (Utilities|GetDisplayName _returnvalue))
  (Pawn|Possess (Game|GetPlayerController 0) _returnvalue)
  (Transformation|SetActorLocation _returnvalue (Transformation|GetWorldLocation (Variables|Default|GetstartLocation)) false false))

(event OnComponentEndOverlap(Entercurve)
  (params (OverlappedComponent :type Primitive%20Component%20Object%20Reference) (OtherActor :type Actor%20Object%20Reference) (OtherComp :type Primitive%20Component%20Object%20Reference) (OtherBodyIndex :type Integer))
  (bind _returnvalue (Actor|GetActorOfClass "/Game/WaterElements/Fish.Fish_C"))
  (Default|MoveinJetstream _returnvalue))

(event EventBeginPlay)

(event Collision|EventActorBeginOverlap
  (params (OtherActor :type Actor%20Object%20Reference)))

(event EventTick
  (params (DeltaSeconds :type Float%20%28single-precision%29)))

(fn ConstructionScript)