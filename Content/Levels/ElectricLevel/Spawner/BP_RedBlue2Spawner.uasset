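; BP_RedBlue2Spawner spawns red/blue rhythm targets for the Electric level, alternating the color with each spawn.
; SpawnRedBlue creates a triple-scale BP_RedBlueRythmTarget at SpawnPoint, sets itself as Spawner, then starts the target with the given delay and current color flag.
; Each target is added to BallSpawned before the flag flips.
; BeginPlay only calls the parent implementation.
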(event EventBeginPlay
  (|CallParentFunction))

(event Collision|EventActorBeginOverlap
  (params (OtherActor :type Actor%20Object%20Reference)))

(event EventTick
  (params (DeltaSeconds :type Float%20%28single-precision%29)))

(fn ConstructionScript)

(fn SpawnRedBlue
  (params (TimeDelay :type Float%20%28double-precision%29))
  (bind _returnvalue (Game|SpawnActorfromClass "/Game/Levels/ElectricLevel/Elec_Rythm_Object/BP_RedBlueRythmTarget.BP_RedBlueRythmTarget_C" (Math|Transform|MakeTransform (Transformation|GetWorldLocation (Variables|Default|GetSpawnPoint)) "0, 0, 0" "3.000000,3.000000,3.000000") "Undefined" 0 0))
  (Variables|/Game/Levels/ElectricLevel/Elec_Rythm_Object/BP_RythmTarget.BP_RythmTarget_C|SetSpawner _returnvalue self)
  (Default|StartRedBlueTarget _returnvalue TimeDelay (Variables|Default|GettoSpawnBlue))
  (Utilities|Set|Add (Variables|Default|GetBallSpawned) _returnvalue)
  (Variables|Default|SettoSpawnBlue (not (Variables|Default|GettoSpawnBlue))))