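; BP_CarSpawner spawns and manages a batch of cars on a shared track in the Electric level, through functions with no callers in this file.
; SpawnCar creates sixteen cars with evenly staggered start offsets shifted by a time delay, and also overrides the player character's minimum analog walk speed and braking friction.
; StartCar moves every stored car, while RemoveCar destroys them and resets the list.
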(event EventBeginPlay)

(event Collision|EventActorBeginOverlap
  (params (OtherActor :type Actor%20Object%20Reference)))

(event EventTick
  (params (DeltaSeconds :type Float%20%28single-precision%29)))

(fn ConstructionScript)

(fn SpawnCar
  (params (timeDelay :type Float%20%28double-precision%29))
  (bind _returnvalue (Game|GetPlayerCharacter 0))
  (bind _charactermovement (Variables|/Script/Engine.Character|GetCharacterMovement _returnvalue))
  (Development|PrintString "ssssss" true true "(R=0.000000,G=0.660000,B=1.000000,A=1.000000)" 11111.0)
  (for _index (range 0 15)
    (bind _returnvalue_2 (Game|SpawnActorfromClass "/Game/Levels/Elec_Ian/Elec3/Car.Car_C" (Math|Transform|MakeTransform "0, 0, 0" "0, 0, 0" "1.000000,1.000000,1.000000") "Undefined" 0 0))
    (Variables|/Game/Levels/Elec_Ian/Elec3/Car.Car_C|SetCarStartOffset _returnvalue_2 (+ (* (Math|Conversions|ToFloat(Integer) _index) 0.042) (* timeDelay (/ 1.0 3e+02))))
    (Variables|/Game/Levels/Elec_Ian/Elec3/Car.Car_C|SetCarTrack _returnvalue_2 (Variables|Default|GetCarTrack))
    (Utilities|Array|Add (Variables|Default|GetCars) _returnvalue_2))
  (Variables|/Script/Engine.CharacterMovementComponent|SetMinAnalogWalkSpeed _charactermovement 1.25e+03)
  (Variables|/Script/Engine.CharacterMovementComponent|SetBrakingFrictionFactor _charactermovement 1e+02))

(fn StartCar
  (for _array_element (Variables|Default|GetCars)
    (Default|MoveCar _array_element)))

(fn RemoveCar
  (for _array_element (Variables|Default|GetCars)
    (Actor|DestroyActor _array_element))
  (Variables|Default|SetCars (LocalVariables|GetEmpty%20Cars)))