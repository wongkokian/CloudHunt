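; Main NPC Blueprint that gives different dialogue on first and repeat interactions and animates when the player is near.
; Interact passes the Beginning messages until Counter reaches the last index, then switches to Repeat, and calls the parent Interact each time.
; Box overlap with ALS_Player loops a talking animation on the skeletal mesh, and leaving returns it to a looping idle.
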(event OnComponentBeginOverlap(Box)
  (params (OverlappedComponent :type Primitive%20Component%20Object%20Reference) (OtherActor :type Actor%20Object%20Reference) (OtherComp :type Primitive%20Component%20Object%20Reference) (OtherBodyIndex :type Integer) (bFromSweep :type Boolean) (SweepResult :type Hit%20Result%20Structure%20%28by%20ref%29))
  (Utilities|Casting|CastToALS_Player OtherActor)
  (Components|Animation|PlayAnimation (Variables|Default|GetSkeletalMesh) "/Game/NPC_Character_Models/Erika/Talking-5_Anim_mixamo_com.Talking-5_Anim_mixamo_com" true))

(event OnComponentEndOverlap(Box)
  (params (OverlappedComponent :type Primitive%20Component%20Object%20Reference) (OtherActor :type Actor%20Object%20Reference) (OtherComp :type Primitive%20Component%20Object%20Reference) (OtherBodyIndex :type Integer))
  (Utilities|Casting|CastToALS_Player OtherActor)
  (Components|Animation|PlayAnimation (Variables|Default|GetSkeletalMesh) "/Game/NPC_Character_Models/Erika/Unarmed_Idle_01-2_Anim_mixamo_com.Unarmed_Idle_01-2_Anim_mixamo_com" true))

(event EventBeginPlay
  (|CallParentFunction) ; This node is disabled and will not be called.\nDrag off pins to build functionality.
)

(event Collision|EventActorBeginOverlap
  (params (OtherActor :type Actor%20Object%20Reference))
  (|CallParentFunction OtherActor) ; This node is disabled and will not be called.\nDrag off pins to build functionality.
)

(event EventTick
  (params (DeltaSeconds :type Float%20%28single-precision%29))
  (|CallParentFunction DeltaSeconds) ; This node is disabled and will not be called.\nDrag off pins to build functionality.
)

(event EventInteract
  (bind _beginning (Variables|Default|GetBeginning))
  (if (Variables|Default|GetFirstInteract)
    (CallFunction|SetMessages _beginning)
    (if (== (Variables|Default|Getcounter) (- (Utilities|Array|Length _beginning) 1))
      (Variables|Default|SetFirstInteract false))
    (else
      (CallFunction|SetMessages (Variables|Default|GetRepeat))))
  (|CallParentFunction))

(fn ConstructionScript
  (|CallParentFunction))