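; BP_FireDamageable is a timed hit target in the boss fire attack that damages the Boss when hit.
; StartTarget billboards it toward the player and runs a timeline that scales Plane1 over twice the given delay, then destroys it.
; The first Hit hides it, disables collision, plays effect and sound, and applies damage scaled by timing accuracy, peaking at the delay mark.
; ChangeColor tints the main plane.
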(event Custom|Start%20Target
  (params (delay :type Float%20%28double-precision%29))
  (CallFunction|StartBillboard (Game|GetPlayerCharacter 0))
  (Variables|Default|SetStart%20Time (Actor|GetGameTimeSinceCreation))
  (bind _output_get (Variables|Default|SetDelay delay))
  (Components|Timeline|SetPlayRate (Variables|Default|GetScale) (/ 1.0 (* _output_get 2.0)))
  (bind _newtrack_0 (Timeline|Scale Play)
    (:Update
      (Transformation|SetRelativeScale3D (Variables|Default|GetPlane1) (Math|Vector|MakeVector _newtrack_0 _newtrack_0 1.0)))
    (:Finished
      (Actor|DestroyActor))))

(event EventBeginPlay)

(event Collision|EventActorBeginOverlap
  (params (OtherActor :type Actor%20Object%20Reference)))

(event EventTick
  (params (DeltaSeconds :type Float%20%28single-precision%29)))

(event EventHit
  (params (isBlueBullet :type Boolean))
  (Utilities|FlowControl|DoOnce false
    (:Completed
      (Niagara|SpawnSystematLocation "/Game/Levels/NS_HitEffectYellow.NS_HitEffectYellow" (Transformation|GetActorLocation) "0, 0,0.000000" "0.010000,0.010000,0.010000")
      (Rendering|SetActorHiddenInGame true)
      (Collision|SetCollisionEnabled (Variables|Default|GetSphere) "NoCollision")
      (Audio|PlaySoundatLocation "/Game/Levels/ElectricLevel/drum_stick_hit_sound.drum_stick_hit_sound" (Transformation|GetActorLocation) "0, 0, 0" 1.0 1.0 0.0 0 0 0 0)
      (bind _effectivedamage (CallFunction|GetEffectiveDamage))
      (Game|Damage|ApplyDamage (Variables|Default|GetBoss) _effectivedamage 0 0))))

(fn ConstructionScript)

(fn ChangeColor
  (params (Color :type Vector))
  (Rendering|Material|SetVectorParameterValueonMaterials (Variables|Default|GetPlane) "BaseColor" Color))

(fn GetEffectiveDamage
  (bind _accuracy (CallFunction|GetAccuracy))
  (return (* (Variables|Default|GetDamage) _accuracy)))

(fn GetAccuracy
  (bind _delay (Variables|Default|GetDelay))
  (return (- 1.0 (/ (Math|Float|Absolute(Float) (- (- (Actor|GetGameTimeSinceCreation) (Variables|Default|GetStart%20Time)) _delay)) _delay))))