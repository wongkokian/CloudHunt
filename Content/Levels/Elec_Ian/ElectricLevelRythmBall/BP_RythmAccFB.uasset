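; BP_RythmAccFB is a short-lived floating text actor that shows accuracy feedback in the electric level's rhythm ball section.
; UpdateText uses Acc2Text to scale an accuracy value into an index of AccuracyTexts and set the label, then destroys the actor after Duration.
; Tick turns the actor to face the player character each frame.
; Acc2Text also prints the scaled value for debugging, and the index is not clamped.
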(event Custom|UpdateText
  (params (Acc :type Float%20%28double-precision%29))
  (CallFunction|Acc2Text Acc)
  (Utilities|FlowControl|Delay (Variables|Default|GetDuration))
  (Actor|DestroyActor))

(event EventBeginPlay)

(event Collision|EventActorBeginOverlap
  (params (OtherActor :type Actor%20Object%20Reference)))

(event EventTick
  (params (DeltaSeconds :type Float%20%28single-precision%29))
  (Transformation|SetActorRotation (Math|Rotator|FindLookatRotation (Transformation|GetActorLocation) (Transformation|GetActorLocation (Game|GetPlayerCharacter 0)))))

(fn ConstructionScript)

(fn Acc2Text
  (params (Acc :type Float%20%28double-precision%29))
  (bind _accuracytexts (Variables|Default|GetAccuracyTexts))
  (bind _returnvalue (Utilities|Array|Length _accuracytexts))
  (bind _returnvalue_2 (* Acc _returnvalue))
  (Development|PrintString (Utilities|String|ToString(Float) _returnvalue_2) true true "(R=0.160940,G=1.000000,B=0.060000,A=1.000000)")
  (Rendering|Components|TextRender|SetText (Variables|Default|Gettext) (Utilities|Array|Get(acopy) (Variables|Default|GetAccuracyTexts) (Math|Float|Floor _returnvalue_2))))