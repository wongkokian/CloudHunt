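; BP_Celebration is a celebration effect that plays a 2D sound on BeginPlay and launches fireworks continuously.
; SpawnStuff spawns one of three firework Niagara systems at random, then calls itself after a short delay, looping without a stop condition.
; GetRandomLocation scatters spawns around the actor in X and Y within Radius, but returns the random angle as Z rather than the actor's height.
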(event Custom|Spawn%20stuff
  (bind _loc (CallFunction|GetRandomLocation))
  (switch int (Math|Random|RandomIntegerinRange 0 2)
    (:Default
      (Niagara|SpawnSystematLocation "/Game/NS_FireWorks.NS_FireWorks" _loc :!label _label))
    (:0
      (goto _label))
    (:1
      (Niagara|SpawnSystematLocation "/Game/NS_FireWorks_2.NS_FireWorks_2" _loc))
    (:2
      (Niagara|SpawnSystematLocation "/Game/NS_FireWorks_3.NS_FireWorks_3" _loc)))
  (Utilities|FlowControl|Delay 0.45)
  (CallFunction|SpawnStuff))

(event EventBeginPlay
  (Audio|PlaySound2D "/Game/gewonnen-87838.gewonnen-87838" 1.0 1.0 0.0 0 0)
  (CallFunction|SpawnStuff))

(event Collision|EventActorBeginOverlap
  (params (OtherActor :type Actor%20Object%20Reference)))

(event EventTick
  (params (DeltaSeconds :type Float%20%28single-precision%29)))

(fn ConstructionScript)

(fn GetRandomLocation
  (bind _returnvalue (Transformation|GetActorLocation))
  (bind _returnvalue_2 (Math|Random|RandomFloat))
  (bind _radius (Variables|Default|GetRadius))
  (bind _returnvalue_3 (* _radius _returnvalue_2))
  (bind _output_get (LocalVariables|Settheta (Math|Random|RandomFloatinRange 0.0 6.28)))
  (return (Math|Vector|MakeVector (- (.x _returnvalue) (* (Math|Trig|Cos(Radians) (LocalVariables|Gettheta)) _returnvalue_3)) (- (.y _returnvalue) (* (Math|Trig|Sin(Radians) (LocalVariables|Gettheta)) _returnvalue_3)) _output_get)))