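; Teleport bubble that ends the water level when the ALS player character overlaps its sphere, sending the player back to WorldLevel.
; On overlap it clears the character's in-water state, resets time dilation and gravity, and removes Transform_Key widgets.
; It then passes the WaterLevelScoreManager score, scaled down, to CHGameInstance for one track and opens WorldLevel by name.
; An in-level Teleport call remains in the graph but is disconnected.
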(event OnComponentBeginOverlap(Sphere)
  (params (OverlappedComponent :type Primitive%20Component%20Object%20Reference) (OtherActor :type Actor%20Object%20Reference) (OtherComp :type Primitive%20Component%20Object%20Reference) (OtherBodyIndex :type Integer) (bFromSweep :type Boolean) (SweepResult :type Hit%20Result%20Structure%20%28by%20ref%29))
  (bind _asals_anim_man_character_bp (Utilities|Casting|CastToALS_AnimMan_CharacterBP OtherActor))
  (Variables|/Game/AdvancedLocomotionV4/Blueprints/CharacterLogic/ALS_AnimMan_CharacterBP.ALS_AnimMan_CharacterBP_C|Setis_in_water _asals_anim_man_character_bp false)
  (Variables|/Script/Engine.Actor|SetCustomTimeDilation _asals_anim_man_character_bp 1.0)
  (Variables|/Script/Engine.CharacterMovementComponent|SetGravityScale (Variables|/Script/Engine.Character|GetCharacterMovement _asals_anim_man_character_bp) 1.0)
  (bind _foundwidgets (Widget|GetAllWidgetsOfClass "/Game/WaterElements/Transform_Key_Widget.Transform_Key_Widget_C" true))
  (Widget|RemovefromParent _foundwidgets)
  (bind _outactors (Actor|GetAllActorsOfClass "/Game/WaterElements/WaterLevelScoreManager.WaterLevelScoreManager_C"))
  (bind _aschgame_instance (Utilities|Casting|CastToCHGameInstance (Game|GetGameInstance)))
  (Default|UpdateScore _aschgame_instance (/ (Variables|/Game/WaterElements/WaterLevelScoreManager.WaterLevelScoreManager_C|GetScore (Utilities|Array|Get(acopy) _outactors)) 1e+02) "NewEnumerator2")
  (Game|OpenLevel(byName) "WorldLevel"))

(event EventBeginPlay)

(event Collision|EventActorBeginOverlap
  (params (OtherActor :type Actor%20Object%20Reference)))

(event EventTick
  (params (DeltaSeconds :type Float%20%28single-precision%29)))

(fn ConstructionScript)