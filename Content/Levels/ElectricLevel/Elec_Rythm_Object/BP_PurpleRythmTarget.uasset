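; BP_PurpleRythmTarget is a two-stage rhythm target that extends a parent target class in the Electric level.
; A timeline scales the green-tinted first target over the first delay, registering a miss and destroying the actor if it finishes.
; Pew stops that timeline, swaps visibility to the second target and starts it with the leftover time plus the second delay, preserving the rhythm's timing.
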(event Custom|Start_Purple_Target
  (params (Delay%201 :type Float%20%28double-precision%29) (Delay%202 :type Float%20%28double-precision%29))
  (CallFunction|StartBillboard)
  (Variables|Default|SetDelay_2 Delay%202)
  (Components|Timeline|SetPlayRate (Variables|Default|GetFirst%20Target) (/ 1.0 Delay%201))
  (bind _scale (Timeline|First%20Target Play)
    (:Update
      (Transformation|SetRelativeScale3D (Variables|Default|GetTarget1) (Math|Vector|MakeVector _scale _scale 1.0)))
    (:Finished
      (CallFunction|MissTarget)
      (Actor|DestroyActor))))

(event Custom|Pew
  (bind _first_target (Variables|Default|GetFirst%20Target))
  (Audio|Components|Audio|Stop (Variables|Default|GetFirst%20Target))
  (Development|SetHiddeninGame (Variables|Default|GetTarget) false false)
  (Development|SetHiddeninGame (Variables|Default|GetTarget1) true false)
  (CallFunction|StartTarget (+ (* (- 1.0 (Components|Timeline|GetPlaybackPosition _first_target)) (/ 1.0 (Components|Animation|GetPlayRate _first_target))) (Variables|Default|GetDelay_2))))

(event EventBeginPlay
  (|CallParentFunction)
  (bind _asbp_target (Utilities|Casting|CastToBP_Target (Variables|/Script/Engine.ChildActorComponent|GetChildActor (Variables|Default|GetTarget1))))
  (Default|ChangeColor _asbp_target "0,1.000000, 0"))

(event Collision|EventActorBeginOverlap
  (params (OtherActor :type Actor%20Object%20Reference)))

(event EventHit
  (params (isBlueBullet :type Boolean))
  (|CallParentFunction false))

(fn ConstructionScript)