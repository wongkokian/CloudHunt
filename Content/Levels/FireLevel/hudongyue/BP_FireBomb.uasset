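; BP_FireBomb is a collectible colored bomb in the fire level that hands its color to a wall block when picked up.
; On BeginPlay it caches the first BP_WallBlock found and sets the BombType material to match its ColorType.
; Any overlap on its StaticMesh prints a debug message and calls CollectBomb, which passes the color to the wall's ReceiveABomb and destroys the bomb.
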(event OnComponentBeginOverlap(StaticMesh)
  (params (OverlappedComponent :type Primitive%20Component%20Object%20Reference) (OtherActor :type Actor%20Object%20Reference) (OtherComp :type Primitive%20Component%20Object%20Reference) (OtherBodyIndex :type Integer) (bFromSweep :type Boolean) (SweepResult :type Hit%20Result%20Structure%20%28by%20ref%29))
  (Development|PrintString "collect a bomb")
  (CallFunction|CollectBomb))

(event EventBeginPlay
  (bind _bombtype (Variables|Default|GetBombType))
  (bind _outactors (Actor|GetAllActorsOfClass "/Game/Levels/FireLevel/hudongyue/BP_WallBlock.BP_WallBlock_C"))
  (Variables|Default|SetWallBlock (Utilities|Array|Get(acopy) _outactors))
  (switch Utilities|FlowControl|Switch|SwitchonBombType (Variables|Default|GetColorType)
    (:NewEnumerator0
      (Rendering|Material|SetMaterial _bombtype 0 "/Game/Levels/ElectricLevel/BP_Trace_Red.BP_Trace_Red"))
    (:NewEnumerator1
      (Rendering|Material|SetMaterial _bombtype 0 "/Game/Levels/ElectricLevel/BP_Trace_Blue.BP_Trace_Blue"))
    (:NewEnumerator2
      (Rendering|Material|SetMaterial _bombtype 0 "/Game/BuildingBlocks/materials/appleTree_surface.appleTree_surface"))
    (:NewEnumerator3
      (Rendering|Material|SetMaterial _bombtype 0 "/Game/BuildingBlocks/materials/appleTree_stem.appleTree_stem"))
    (:NewEnumerator4
      (Rendering|Material|SetMaterial _bombtype 0 "/Game/BuildingBlocks/meshes/ShoudaMesh/FlowerAndGrass/Blossoms01.Blossoms01"))))

(event Collision|EventActorBeginOverlap
  (params (OtherActor :type Actor%20Object%20Reference)))

(event EventTick
  (params (DeltaSeconds :type Float%20%28single-precision%29)))

(fn ConstructionScript)

(fn CollectBomb
  (Default|ReceiveABomb (Variables|Default|GetWallBlock) (Variables|Default|GetColorType))
  (Actor|DestroyActor))