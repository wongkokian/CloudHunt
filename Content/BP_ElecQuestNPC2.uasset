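; BP_ElecQuestNPC2 is a quest NPC whose messages depend on whether an electricity quest is complete.
; On interaction it runs the parent behavior, then reads IsComplete from its ElecController and sets either the completed or incomplete message set.
; Because the update follows the parent Interact call, messages refresh only after each interaction is handled.
; BeginPlay and overlap end only forward to the parent.
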(event Custom|Update%20%20Message
  (if (Variables|/Game/Levels/ElectricLevel/ElecLevel/ElectricLevelController.ElectricLevelController_C|GetisComplete (Variables|Default|GetElecController))
    (CallFunction|SetMessages (Variables|Default|GetCompleted%20Messages))
    (else
      (CallFunction|SetMessages (Variables|Default|GetIncomplete%20Messages)))))

(event EventBeginPlay
  (|CallParentFunction))

(event EventInteract
  (|CallParentFunction)
  (CallFunction|UpdateMessage))

(event Collision|EventActorEndOverlap
  (params (OtherActor :type Actor%20Object%20Reference))
  (|CallParentFunction 0))

(fn ConstructionScript)