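; BP_DriveableSpawner is a spawner that places driveable targets along the spline of a referenced driveable car.
; On BeginPlay it precomputes spawn transforms by sampling the car's location along its spline at successive time steps.
; Each SpawnTarget call spawns a BP_DriveableTarget at the current beat's transform, randomly shifts it between three lateral lanes, starts it with a delay and advances the beat.
; It also rounds the parent's average accuracy.
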(event EventBeginPlay
  (|CallParentFunction)
  (CallFunction|Init))

(event Collision|EventActorBeginOverlap
  (params (OtherActor :type Actor%20Object%20Reference))
  (|CallParentFunction OtherActor) ; This node is disabled and will not be called.\nDrag off pins to build functionality.
)

(fn ConstructionScript
  (|CallParentFunction))

(fn Init
  (for _index (range 2 50)
    (bind _transform (Default|LocationatSplineatTime (Variables|Default|GetDriveableCar) (Math|Conversions|ToFloat(Integer) (+ _index 1))))
    (Utilities|Array|Add (Variables|Default|GetSpawn%20Transform) _transform)))

(fn SpawnTarget
  (params (TimeDelay :type Float%20%28double-precision%29))
  (bind _returnvalue (Game|SpawnActorfromClass "/Game/Levels/ElectricLevel/BP_DriveableTarget.BP_DriveableTarget_C" (Utilities|Array|Get(acopy) (Variables|Default|GetSpawn%20Transform) (Variables|Default|GetBeat)) "Undefined" 0 0))
  (Transformation|AddActorLocalOffset _returnvalue (Math|Vector|MakeVector 0.0 (Math|Conversions|ToFloat(Integer) (* (Math|Random|RandomIntegerinRange -1 1) 500)) 0.0) false false)
  (Variables|/Game/Levels/ElectricLevel/BP_DriveableTarget.BP_DriveableTarget_C|SetCar%20Reference _returnvalue (Variables|Default|GetDriveableCar))
  (Variables|/Game/Levels/ElectricLevel/Elec_Rythm_Object/BP_RythmTarget.BP_RythmTarget_C|SetSpawner _returnvalue self)
  (Default|StartTarget _returnvalue TimeDelay)
  (Utilities|Set|Add (Variables|Default|GetBallSpawned) _returnvalue)
  (Math|Integer|IncrementInt (Variables|Default|GetBeat)))

(fn GetAverageAccuracy
  (bind _average_accuray (|CallParentFunction))
  (return (Math|Conversions|ToFloat(Integer) (Math|Float|Round _average_accuray))))