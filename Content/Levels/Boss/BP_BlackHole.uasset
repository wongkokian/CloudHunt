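; BP_BlackHole is a boss-level hazard actor that appears as a scaling sphere and damages the player on contact.
; On BeginPlay, a timeline drives the uniform world scale of Sphere1, and the actor destroys itself when the timeline finishes.
; An overlapping ALS_Player receives an explosion hit message with very high damage, with the black hole as the source.
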(event EventBeginPlay
  (bind _newtrack_2 (Timeline|BLACKGHOLE Play)
    (:Update
      (Transformation|SetWorldScale3D (Variables|Default|GetSphere1) (Math|Vector|MakeVector _newtrack_2 _newtrack_2 _newtrack_2)))
    (:Finished
      (Actor|DestroyActor))))

(event Collision|EventActorBeginOverlap
  (params (OtherActor :type Actor%20Object%20Reference))
  (if (== (Utilities|GetClass OtherActor) "/Game/AdvancedLocomotionV4/Blueprints/CharacterLogic/ALS_Player.ALS_Player_C")
    (bind _asals_player (Utilities|Casting|CastToALS_Player OtherActor))
    (Class|CLMBPIDamageable|OnExplosionHit(Message) _asals_player self 1e+03)))

(event EventTick
  (params (DeltaSeconds :type Float%20%28single-precision%29)))

(fn ConstructionScript)