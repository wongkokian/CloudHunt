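; Base electric projectile for the monster system that damages the player on contact.
; A sphere overlap with an ALS_Player hides it, disables collision, calls OnExplosionHit with its damage, spawns an explosion emitter and expires shortly after, ignoring other actors.
; A looping timer, rather than Tick, billboards the plane mesh toward the player camera.
; InitializeProjectile sets the movement component's initial and max speed.
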(event Custom|PorjectileHit
  (params (OverlappedComponent :type Primitive%20Component%20Object%20Reference) (OtherActor :type Actor%20Object%20Reference) (OtherComp :type Primitive%20Component%20Object%20Reference) (OtherBodyIndex :type Integer) (bFromSweep :type Boolean) (SweepResult :type Hit%20Result%20Structure%20%28by%20ref%29))
  (bind _self self)
  (if (Utilities|ClassIsChildOf (Utilities|GetClass OtherActor) "/Game/AdvancedLocomotionV4/Blueprints/CharacterLogic/ALS_Player.ALS_Player_C")
    (Rendering|SetActorHiddenInGame true)
    (Collision|SetActorEnableCollision false)
    (bind _asals_player (Utilities|Casting|CastToALS_Player OtherActor))
    (Default|OnExplosionHit _asals_player _self (Variables|Default|GetDamage))
    (Effects|SpawnEmitteratLocation "/Game/StarterContentMin/Particles/P_Explosion.P_Explosion" (Transformation|GetActorLocation _self))
    (Actor|SetLifeSpan 1.0)))

(event EventBeginPlay
  (Collision|BindEventtoOnComponentBeginOverlap (Variables|Default|GetSphere) (delegate Custom|PorjectileHit))
  (Utilities|Time|SetTimerbyFunctionName 0 "FacePlayer" 0.1 true))

(event EventTick
  (params (DeltaSeconds :type Float%20%28single-precision%29)))

(fn ConstructionScript)

(fn FacePlayer
  (bind _returnvalue (Game|GetPlayerCameraManager 0))
  (bind _returnvalue_2 (Transformation|GetActorLocation))
  (bind _returnvalue_3 (Camera|GetCameraLocation _returnvalue))
  (bind _returnvalue_4 (- _returnvalue_3 _returnvalue_2))
  (bind _returnvalue_5 (Math|Vector|Normalize _returnvalue_4))
  (bind _returnvalue_6 (Math|Conversions|RotationFromXVector _returnvalue_5))
  (Transformation|SetWorldRotation (Variables|Default|GetPlane) (Math|Rotator|MakeRotator (.roll _returnvalue_6) (+ (.pitch _returnvalue_6) 9e+01) (.yaw _returnvalue_6)) false false))

(fn InitializeProjectile
  (params (speed :type Float%20%28double-precision%29))
  (bind _projectilemovement (Variables|Default|GetProjectileMovement))
  (bind _output_get (Variables|/Script/Engine.ProjectileMovementComponent|SetInitialSpeed _projectilemovement speed))
  (Variables|/Script/Engine.ProjectileMovementComponent|SetMaxSpeed _projectilemovement _output_get))