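; Fire-level trigger actor that launches a burst of fireballs when any actor begins overlapping it.
; On overlap it spawns a FireSphere_long at each of its four point components' world transforms, playing the BigFireBall sound at the trigger's own location before each spawn.
; The event has no actor filter, delay or one-shot guard, so every new overlap repeats the full burst.
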(event Collision|EventActorBeginOverlap
  (params (OtherActor :type Actor%20Object%20Reference))
  (Audio|SpawnSoundatLocation "/Game/Levels/FireLevel/ShoudaFX/Sound/BigFireBall.BigFireBall" (Transformation|GetActorLocation) "0, 0, 0" 1.0 1.0 0.0 0 0)
  (Game|SpawnActorfromClass "/Game/Levels/FireLevel/ShoudaFX/BP/FireSphere_long.FireSphere_long_C" (Transformation|GetWorldTransform (Variables|Default|GetPOINT2)) "Undefined" 0 0)
  (Audio|SpawnSoundatLocation "/Game/Levels/FireLevel/ShoudaFX/Sound/BigFireBall.BigFireBall" (Transformation|GetActorLocation) "0, 0, 0" 1.0 1.0 0.0 0 0)
  (Game|SpawnActorfromClass "/Game/Levels/FireLevel/ShoudaFX/BP/FireSphere_long.FireSphere_long_C" (Transformation|GetWorldTransform (Variables|Default|GetPOINT1)) "Undefined" 0 0)
  (Audio|SpawnSoundatLocation "/Game/Levels/FireLevel/ShoudaFX/Sound/BigFireBall.BigFireBall" (Transformation|GetActorLocation) "0, 0, 0" 1.0 1.0 0.0 0 0)
  (Game|SpawnActorfromClass "/Game/Levels/FireLevel/ShoudaFX/BP/FireSphere_long.FireSphere_long_C" (Transformation|GetWorldTransform (Variables|Default|GetPOINT)) "Undefined" 0 0)
  (Audio|SpawnSoundatLocation "/Game/Levels/FireLevel/ShoudaFX/Sound/BigFireBall.BigFireBall" (Transformation|GetActorLocation) "0, 0, 0" 1.0 1.0 0.0 0 0)
  (Game|SpawnActorfromClass "/Game/Levels/FireLevel/ShoudaFX/BP/FireSphere_long.FireSphere_long_C" (Transformation|GetWorldTransform (Variables|Default|GetPOINT3)) "Undefined" 0 0))

(fn ConstructionScript)