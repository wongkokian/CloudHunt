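; BP_MusicTree is an interactable music tree for an Electric Level sub-quest, with a monument, an orb and audio.
; While active, interacting passes its State to Parent, whose returned result decides whether the orb is revealed.
; Activate enables query collision and plays audio; Complete shows the orb, stops audio and disables interaction.
; Highlighting toggles the monument's custom depth; material swaps are left unconnected.
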(event EventInteract
  (if (Variables|Default|GetisActive)
    (CallFunction|UpdateParent)
    (|CallParentFunction)))

(fn ConstructionScript)

(fn UpdateParent
  (bind _correct_sequence (Default|UpdateState (Variables|Default|Getparent) (Variables|Default|Getstate)))
  (CallFunction|Update _correct_sequence))

(fn Update
  (params (to%20update :type Boolean))
  (if to%20update
    (Development|SetHiddeninGame (Variables|Default|GetOrb) false false)))

(fn DeactivateAppearance
  (Development|SetHiddeninGame (Variables|Default|GetOrb) true false))

(fn DeactivateSound
  (Audio|Components|Audio|Stop (Variables|Default|GetAudio)))

(fn Complete
  (CallFunction|ActivateAppearanceComplete)
  (CallFunction|DeactivateSound)
  (Variables|Default|SetisActive false)
  (Collision|SetCollisionEnabled (Variables|Default|GetCollision) "NoCollision"))

(fn Activate
  (Variables|Default|SetisActive true)
  (Collision|SetCollisionEnabled (Variables|Default|GetCollision) "QueryOnly")
  (Audio|Components|Audio|Play (Variables|Default|GetAudio) 0.0))

(fn ActivateAppearanceComplete
  (Development|SetHiddeninGame (Variables|Default|GetOrb) false false))

(fn UntoggleHighlight
  (|CallParentFunction)
  (Rendering|SetRenderCustomDepth (Variables|Default|GetMonument) false))

(fn ToggleHighlight
  (|CallParentFunction)
  (Rendering|SetRenderCustomDepth (Variables|Default|GetMonument) true))