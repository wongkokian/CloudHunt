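; BP_RedBlueRythmTarget is a two-color variant of a rhythm target that only counts hits from a bullet of the matching color.
; Start_RedBlue_Target sets the color, starts the target with the given delay and reveals the blue or red component.
; Hit passes a color match to the parent's hit logic through a DoOnce, which resets on a mismatch so the target can still be hit.
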(event Custom|Start_RedBlue_Target
  (params (Time%20Delay :type Float%20%28double-precision%29) (ToSpawnBlue :type Boolean))
  (bind _output_get (Variables|Default|SetisBlue ToSpawnBlue))
  (CallFunction|StartTarget Time%20Delay)
  (if _output_get
    (Development|SetHiddeninGame (Variables|Default|GetBlue%20Target) false false)
    (else
      (Development|SetHiddeninGame (Variables|Default|GetRed%20Target) false false))))

(event EventBeginPlay
  (|CallParentFunction))

(event Collision|EventActorBeginOverlap
  (params (OtherActor :type Actor%20Object%20Reference)))

(event EventTick
  (params (DeltaSeconds :type Float%20%28single-precision%29)))

(event EventHit
  (params (isBlueBullet :type Boolean))
  (Utilities|FlowControl|DoOnce false :!label _label
    (:Completed
      (if (not (Class|KismetMathLibrary|XORBoolean isBlueBullet (Variables|Default|GetisBlue)))
        (|CallParentFunction false)
        (else
          (goto _label Reset))))))

(fn ConstructionScript)