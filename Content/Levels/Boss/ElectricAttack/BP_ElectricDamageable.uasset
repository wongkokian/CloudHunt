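; Timed blue or magenta target in the boss electric attack that damages the Boss when hit by a bullet of matching color.
; StartTarget starts billboarding toward the player, tints the planes and runs a scale timeline over twice the Delay, destroying the actor when it finishes.
; The first matching Hit hides the target, plays effects and applies damage scaled by timing accuracy, which peaks at Delay and falls off linearly either side.
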(event Custom|Start%20Target
  (params (delay :type Float%20%28double-precision%29) (isBlue :type Boolean))
  (CallFunction|StartBillboard (Game|GetPlayerCharacter 0))
  (bind _output_get (Variables|Default|SetisBlue isBlue))
  (if _output_get
    (CallFunction|ChangeColor "0.000000, 0,1.000000")
    (else
      (CallFunction|ChangeColor "1.000000, 0,1.000000")))
  (Variables|Default|SetStart%20Time (Actor|GetGameTimeSinceCreation))
  (bind _output_get_2 (Variables|Default|SetDelay delay))
  (Components|Timeline|SetPlayRate (Variables|Default|GetScale) (/ 1.0 (* _output_get_2 2.0)))
  (bind _newtrack_0 (Timeline|Scale Play)
    (:Update
      (Transformation|SetRelativeScale3D (Variables|Default|GetPlane1) (Math|Vector|MakeVector _newtrack_0 _newtrack_0 1.0)))
    (:Finished
      (Actor|DestroyActor))))

(event EventBeginPlay)

(event Collision|EventActorBeginOverlap
  (params (OtherActor :type Actor%20Object%20Reference)))

(event EventTick
  (params (DeltaSeconds :type Float%20%28single-precision%29)))

(event EventHit
  (params (isBlueBullet :type Boolean))
  (if (not (Class|KismetMathLibrary|XORBoolean isBlueBullet (Variables|Default|GetisBlue)))
    (Utilities|FlowControl|DoOnce false
      (:Completed
        (if isBlueBullet
          (Niagara|SpawnSystematLocation "/Game/Levels/NS_HitEffectBlue.NS_HitEffectBlue" (Transformation|GetActorLocation) "0, 0, 0" "0.400000,0.400000,0.400000")
          (else
            (Niagara|SpawnSystematLocation "/Game/Levels/NS_HitEffectRed.NS_HitEffectRed" (Transformation|GetActorLocation) "0, 0, 0" "0.400000,0.400000,0.400000")))
        (Rendering|SetActorHiddenInGame true)
        (Collision|SetCollisionEnabled (Variables|Default|GetSphere) "NoCollision")
        (Audio|PlaySoundatLocation "/Game/Levels/ElectricLevel/drum_stick_hit_sound.drum_stick_hit_sound" (Transformation|GetActorLocation) "0, 0, 0" 1.0 1.0 0.0 0 0 0 0)
        (bind _effectivedamage (CallFunction|GetEffectiveDamage))
        (Game|Damage|ApplyDamage (Variables|Default|GetBoss) _effectivedamage 0 0)))))

(fn ConstructionScript)

(fn ChangeColor
  (params (Color :type Vector))
  (Rendering|Material|SetVectorParameterValueonMaterials (Variables|Default|GetPlane) "BaseColor" Color)
  (Rendering|Material|SetVectorParameterValueonMaterials (Variables|Default|GetPlane1) "BaseColor" Color))

(fn GetEffectiveDamage
  (bind _accuracy (CallFunction|GetAccuracy))
  (return (* (Variables|Default|GetDamage) _accuracy)))

(fn GetAccuracy
  (bind _delay (Variables|Default|GetDelay))
  (return (- 1.0 (/ (Math|Float|Absolute(Float) (- (- (Actor|GetGameTimeSinceCreation) (Variables|Default|GetStart%20Time)) _delay)) _delay))))