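; BP_BlueBall is a short-lived ball actor that awards score to BP_Sprite when destroyed through DestroyBall.
; On BeginPlay it caches the first BP_Sprite and self-destructs after a delay, or earlier, without scoring, on sphere hit or overlap.
; DestroyBall, not called within this Blueprint, adds score and spawns explosion sound and particles before destroying the actor.
; Movement logic, including randomized speeds and a timeline, is disconnected, so nothing here moves the ball.
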(event OnComponentHit(Sphere)
  (params (HitComponent :type Primitive%20Component%20Object%20Reference) (OtherActor :type Actor%20Object%20Reference) (OtherComp :type Primitive%20Component%20Object%20Reference) (NormalImpulse :type Vector :default "0, 0, 0") (Hit :type Hit%20Result%20Structure%20%28by%20ref%29))
  (Actor|DestroyActor))

(event OnComponentBeginOverlap(Sphere)
  (params (OverlappedComponent :type Primitive%20Component%20Object%20Reference) (OtherActor :type Actor%20Object%20Reference) (OtherComp :type Primitive%20Component%20Object%20Reference) (OtherBodyIndex :type Integer) (bFromSweep :type Boolean) (SweepResult :type Hit%20Result%20Structure%20%28by%20ref%29))
  (Actor|DestroyActor))

(event EventBeginPlay
  (Variables|Default|SetBallMovingSpeedX (Math|Random|RandomFloatinRange -1e+01 1e+01))
  (Variables|Default|SetBallMovingSpeedY (Math|Random|RandomFloatinRange -1e+01 1e+01))
  (Variables|Default|SetBallMovingSpeedZ 1e+01)
  (bind _outactors (Actor|GetAllActorsOfClass "/Game/Levels/FireLevel/hudongyue/BP_Sprite.BP_Sprite_C"))
  (Variables|Default|SetSprite (Utilities|Array|Get(acopy) _outactors))
  (Utilities|FlowControl|Delay 5.0)
  (Actor|DestroyActor))

(event Collision|EventActorBeginOverlap
  (params (OtherActor :type Actor%20Object%20Reference)))

(event EventTick
  (params (DeltaSeconds :type Float%20%28single-precision%29)))

(fn ConstructionScript)

(fn DestroyBall
  (bind _returnvalue (Transformation|GetActorLocation))
  (Development|PrintString "The blue ball will be destroyed")
  (Default|AddScore (Variables|Default|GetSprite))
  (Audio|SpawnSoundatLocation "/Game/StarterContent/Audio/Explosion01.Explosion01" _returnvalue "0, 0, 0" 1.0 1.0 0.0 0 0)
  (Effects|SpawnEmitteratLocation "/Game/StarterContent/Particles/P_Explosion.P_Explosion" _returnvalue)
  (Actor|DestroyActor))