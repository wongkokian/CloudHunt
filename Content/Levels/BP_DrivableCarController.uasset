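; Phase controller that hands the player over to a drivable car during a level.
; TriggerPhase possesses the car and hides the player character before running the parent phase logic.
; A sequencer Complete event re-enables automatic camera lookup and sets the view target back to the player controller.
; Flower target spawning is unfinished: Init's loop over spawn times is empty, SpawnTarget is never run, and RandomOffset is not called.
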(event EventBeginPlay
  (CallFunction|Init))

(event Collision|EventActorBeginOverlap
  (params (OtherActor :type Actor%20Object%20Reference)))

(event EventTick
  (params (DeltaSeconds :type Float%20%28single-precision%29)))

(event Custom|Complete
  (bind _returnvalue (Game|GetPlayerController 0))
  (Variables|Default|SetbFindCameraComponentWhenViewTarget true)
  (Game|Player|SetViewTargetwithBlend _returnvalue _returnvalue 0.0 "VTBlend_Linear" 0.0 false))

(fn ConstructionScript)

(fn TriggerPhase
  (Default|PossessCar (Variables|Default|GetDriveableCar))
  (Rendering|SetActorHiddenInGame (Game|GetPlayerCharacter 0) true)
  (|CallParentFunction))

(fn Init
  (for _array_element (Variables|Default|GetSpawn%20Time)
    _))

(fn SpawnTarget
  (for (_array_element _array_index) (Variables|Default|GetSpawn%20Location)
    (Game|SpawnActorfromClass "/Game/BuildingBlocks/flower_bp.flower_bp_C" (Math|Transform|MakeTransform _array_element (Utilities|Array|Get(acopy) (Variables|Default|GetSpawn%20Rotation) _array_index) "1.000000,1.000000,1.000000") "Undefined" 0 0)))

(fn RandomOffset
  (return (Math|Conversions|ToFloat(Integer) (* (Math|Random|RandomIntegerinRange -1 1) 500))))