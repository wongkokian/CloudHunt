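; Wind controller actor for the birch forest that writes wind settings into the MPC_Wind_Birch material parameter collection.
; It pushes intensity, speed, the negated XY of an Arrow component's forward vector, and that heading as a 0–1 fraction of a turn.
; The update runs in the construction script, then either every Tick or once at BeginPlay, depending on UpdateRuntime.
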(event EventBeginPlay
  (if (not (Variables|Default|GetUpdate%20Runtime))
    (CallFunction|WindParameters)))

(event EventTick
  (params (DeltaSeconds :type Float%20%28single-precision%29))
  (if (Variables|Default|GetUpdate%20Runtime)
    (CallFunction|WindParameters)))

(fn ConstructionScript
  (CallFunction|WindParameters))

(fn WindParameters
  (Rendering|Material|SetScalarParameterValue "/Game/StylizedBirchForest/Materials/MaterialParameterCollections/MPC_Wind_Birch.MPC_Wind_Birch" "WindIntensity" (Variables|Wind|GetWind%20Intensity) :!class /Script/Engine.KismetMaterialLibrary)
  (Rendering|Material|SetScalarParameterValue "/Game/StylizedBirchForest/Materials/MaterialParameterCollections/MPC_Wind_Birch.MPC_Wind_Birch" "WindSpeed" (Variables|Wind|GetWind%20Speed) :!class /Script/Engine.KismetMaterialLibrary)
  (Variables|Default|SetWind%20Direction (Math|Vector|GetForwardVector (Variables|Default|GetArrow)))
  (Rendering|Material|SetVectorParameterValue "/Game/StylizedBirchForest/Materials/MaterialParameterCollections/MPC_Wind_Birch.MPC_Wind_Birch" "WindDirection" (Utilities|Struct|MakeLinearColor (.X (Math|Vector|BreakVector (* (Variables|Default|GetWind%20Direction) -1))) (.Y (Math|Vector|BreakVector (* (Variables|Default|GetWind%20Direction) -1))) 0.0 1.0) :!class /Script/Engine.KismetMaterialLibrary)
  (Rendering|Material|SetScalarParameterValue "/Game/StylizedBirchForest/Materials/MaterialParameterCollections/MPC_Wind_Birch.MPC_Wind_Birch" "WindDirectionRad" (Math|Float|Fraction (/ (Math|Trig|Atan2(Radians) (.X (Math|Vector|BreakVector (Variables|Default|GetWind%20Direction))) (.Y (Math|Vector|BreakVector (Variables|Default|GetWind%20Direction)))) 6.283185)) :!class /Script/Engine.KismetMaterialLibrary))