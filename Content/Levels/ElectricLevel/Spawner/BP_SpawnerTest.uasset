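; BP_SpawnerTest is a test actor in the electric level that exercises two ball spawners and an AI controller.
; After a short delay on BeginPlay it triggers the AI controller's phase, then starts two timers by function name.
; A looping timer has one spawner spawn "Bom" and the other red/blue spawns.
; A one-shot timer later removes all balls from both spawners, without stopping the spawn loop.
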(event EventBeginPlay
  (Utilities|FlowControl|Delay 5.0)
  (Default|TriggerPhase (Variables|Default|GetAi%20Controller))
  (Utilities|Time|SetTimerbyFunctionName 0 "Spawn" 4.0 true)
  (Utilities|Time|SetTimerbyFunctionName 0 "Remove" 2e+01))

(event Collision|EventActorBeginOverlap
  (params (OtherActor :type Actor%20Object%20Reference)))

(event EventTick
  (params (DeltaSeconds :type Float%20%28single-precision%29)))

(fn ConstructionScript)

(fn Spawn
  (Default|SpawnBom (Variables|Default|GetSpawner) 2.0 2.0)
  (Default|SpawnRedBlue (Variables|Default|GetSpawner2) 2.0))

(fn Remove
  (Default|RemoveAllBalls (Variables|Default|GetSpawner))
  (Default|RemoveAllBalls (Variables|Default|GetSpawner2)))