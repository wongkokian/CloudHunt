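; Fire level sprite actor that moves its Cube along a looping spline and has helpers for spawning balls and counting score.
; Tick advances a distance by MovingSpeed, sets the Cube's relative location and yaw from the spline, and restarts at the end.
; GenerateBall spawns a red or blue ball below the Cube, and AddScore increments and prints the score.
; The older timeline movement and timed red/blue spawn loop are disconnected.
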(event EventBeginPlay
  ;[1 1 1] Set Origin Location
  (Variables|Default|SetOriginLocation (Transformation|GetWorldLocation (Variables|Default|GetCube))))

(event Collision|EventActorBeginOverlap
  (params (OtherActor :type Actor%20Object%20Reference)))

(event EventTick
  (params (DeltaSeconds :type Float%20%28single-precision%29))
  (bind _distance (Variables|Default|GetDistance))
  (bind _spline (Variables|Default|GetSpline))
  (bind _returnvalue (Spline|GetTransformatDistanceAlongSpline _spline _distance "Local" false))
  ;[1 1 1] new spline moving
  (Variables|Default|Setdistance (+ (* DeltaSeconds (Variables|Default|GetMovingSpeed)) (Variables|Default|GetDistance)))
  (Transformation|SetRelativeTransform (Variables|Default|GetCube) (Math|Transform|MakeTransform (.location _returnvalue) (Math|Rotator|MakeRotator 0.0 0.0 (.yaw (.rotation _returnvalue))) (Variables|/Script/Engine.SceneComponent|GetRelativeScale3D (Variables|Default|GetCube))) false false)
  (if (> (Variables|Default|GetDistance) (Spline|GetSplineLength (Variables|Default|GetSpline)))
    (Variables|Default|Setdistance 0.0)))

(fn ConstructionScript)

(fn GenerateBall
  (params (BallColor :type ColorChoice%20Enum :default "NewEnumerator0"))
  (bind _cube (Variables|Default|GetCube))
  (bind _returnvalue (Transformation|GetWorldTransform _cube))
  (bind _returnvalue_2 (+ (.location _returnvalue) "0,0.000000,-150.000000"))
  (switch Utilities|FlowControl|Switch|SwitchonColorChoice BallColor
    (:NewEnumerator0
      (Game|SpawnActorfromClass "/Game/Levels/FireLevel/hudongyue/BP_RedBall.BP_RedBall_C" (Math|Transform|MakeTransform _returnvalue_2 (.rotation _returnvalue) "1.000000,1.000000,1.000000") "Undefined" 0 0))
    (:NewEnumerator1
      (Game|SpawnActorfromClass "/Game/Levels/FireLevel/hudongyue/BP_BlueBall.BP_BlueBall_C" (Math|Transform|MakeTransform _returnvalue_2 (.rotation _returnvalue) "1.000000,1.000000,1.000000") "Undefined" 0 0))))

(fn AddScore
  (Variables|Default|SetScore (+ (Variables|Default|GetScore) 1))
  (Development|PrintString (Utilities|String|Append "you have score " (Utilities|String|ToString(Integer) (Variables|Default|GetScore)))))