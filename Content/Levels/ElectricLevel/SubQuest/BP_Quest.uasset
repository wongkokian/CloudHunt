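; Base quest actor for the Electric Level sub-quests that tracks active and completed state and saves completion by quest name through CHGameInstance.
; On BeginPlay it reads the saved status and calls InitComplete, an empty hook, if the quest is already done.
; StartQuest marks it active, CompleteQuest marks it done and reports to the game instance, and UpdateQuestStatus reports the current state.
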(event EventBeginPlay
  (CallFunction|Init))

(event Collision|EventActorBeginOverlap
  (params (OtherActor :type Actor%20Object%20Reference)))

(event EventTick
  (params (DeltaSeconds :type Float%20%28single-precision%29)))

(event EventCompleteQuest
  (bind _output_get (Variables|Default|SetisComplete true))
  (Variables|Default|SetisActive false)
  (bind _aschgame_instance (Utilities|Casting|CastToCHGameInstance (Game|GetGameInstance)))
  (Default|UpdateQuestStatus _aschgame_instance (Variables|Default|GetquestName) _output_get))

(event EventStartQuest
  (Variables|Default|SetisActive true))

(event EventUpdateQuestStatus
  (bind _aschgame_instance (Utilities|Casting|CastToCHGameInstance (Game|GetGameInstance)))
  (Default|UpdateQuestStatus _aschgame_instance (Variables|Default|GetquestName) (Variables|Default|GetisComplete)))

(fn ConstructionScript)

(fn Init
  (bind _aschgame_instance (Utilities|Casting|CastToCHGameInstance (Game|GetGameInstance)))
  (bind _status (Default|GetQuestStatus _aschgame_instance (Utilities|String|StringToName (Variables|Default|GetquestName))))
  (bind _output_get (Variables|Default|SetisComplete _status))
  (if _output_get
    (CallFunction|InitComplete)))

(fn InitComplete)

(fn IsComplete
  (return (Variables|Default|GetisComplete)))