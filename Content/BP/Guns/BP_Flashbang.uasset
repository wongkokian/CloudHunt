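; Flashbang grenade that blinds and deafens the player and sends a flashbang-hit message to nearby pawns when it explodes.
; The full flash needs the grenade recently rendered within flash radius, or an unobstructed trace within inner radius; visible distant blasts only ring ears.
; The flash overrides the first post-process volume with a dynamic material and slows global time.
; A timeline fades effect and slowdown, then restores the saved settings.
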(event Custom|AffectNearbyCharacters
  (bind _sm_grenade (Variables|Default|GetSM%20Grenade))
  (bind _returnvalue (Transformation|GetWorldLocation _sm_grenade))
  (bind (_outhits _returnvalue_2) (Collision|MultiSphereTraceForObjects _returnvalue (+ _returnvalue "1.000000,0,0") (Variables|Default|GetFlash%20Radius) (Utilities|Array|MakeArray "ObjectTypeQuery3") false (Utilities|Array|MakeArray (Game|GetPlayerCharacter 0)) "None"))
  (if _returnvalue_2
    (for _array_element _outhits
      (Utilities|Array|AddUnique (Variables|Default|Getaffected%20actors) (.HitActor (Collision|BreakHitResult _array_element))))
    (for _array_element_2 (Variables|Default|Getaffected%20actors)
      (Class|CLMBPIDamageable|OnFlashBangHit(Message) _array_element_2 "0, 0, 0" (Math|Random|RandomFloatinRange 3.0 5.0)))))

(event EventBeginPlay
  (|CallParentFunction)
  (bind _outactors (Actor|GetAllActorsOfClass "/Script/Engine.PostProcessVolume"))
  (if (> (Utilities|Array|Length _outactors) 0)
    (bind _output_get (Variables|Default|SetPP_Vol (Utilities|Array|Get(acopy) _outactors)))
    (Variables|Default|SetOriginal%20Settings (Variables|/Script/Engine.PostProcessVolume|GetSettings _output_get))))

(event Collision|EventActorBeginOverlap
  (params (OtherActor :type Actor%20Object%20Reference))
  (|CallParentFunction OtherActor) ; This node is disabled and will not be called.\nDrag off pins to build functionality.
)

(event EventTick
  (params (DeltaSeconds :type Float%20%28single-precision%29))
  (|CallParentFunction DeltaSeconds) ; This node is disabled and will not be called.\nDrag off pins to build functionality.
)

(event EventExplodeGrenade
  (bind _returnvalue (Game|GetPlayerCharacter 0))
  (bind _sm_grenade (Variables|Default|GetSM%20Grenade))
  (bind _returnvalue_2 (Transformation|GetWorldLocation _sm_grenade))
  (bind _returnvalue_3 (Transformation|GetActorLocation _returnvalue))
  (|CallParentFunction)
  (CallFunction|AffectNearbyCharacters)
  (if (Class|Actor|WasRecentlyRendered 0.1)
    (if (< (Math|Vector|Distance(Vector) _returnvalue_2 _returnvalue_3) (Variables|Default|GetFlash%20Radius))
      (Audio|Components|Audio|Play (Variables|Default|GetEar_Ringing) 0.0 :!label _label)
      (|EnablePP_Effect)
      (Utilities|Time|SetGlobalTimeDilation 0.1)
      (Utilities|FlowControl|Delay (Math|Float|SelectFloat 0.2 0.1 (< (Math|Vector|Distance(Vector) (Transformation|GetWorldLocation (Variables|Default|GetSM%20Grenade)) (Transformation|GetActorLocation (Game|GetPlayerCharacter 0))) (/ (Variables|Default|GetFlash%20Radius) 2.0))))
      (Audio|Components|Audio|FadeOut (Variables|Default|GetEar_Ringing) 3.0 0.0 "Linear" :!class /Script/Engine.AudioComponent)
      (|FadeOutPPEffect
        (:Finished
          (Variables|/Script/Engine.PostProcessVolume|SetSettings (Variables|Default|GetPP_Vol) (Variables|Default|GetOriginal%20Settings))))
      (else
        (Audio|Components|Audio|Play (Variables|Default|GetEar_Ringing) 0.0)
        (Utilities|FlowControl|Delay 1.0)
        (Audio|Components|Audio|FadeOut (Variables|Default|GetEar_Ringing) 3.0 0.0 "Linear" :!class /Script/Engine.AudioComponent)))
    (else
      (bind (_outhit _returnvalue_4) (Collision|LineTraceByChannel _returnvalue_2 _returnvalue_3 "TraceTypeQuery1" false 0 "None"))
      (if _returnvalue_4
        (if (and (< (.Distance (Collision|BreakHitResult _outhit)) (Variables|Default|GetInner%20Flash%20Radius)) (== (.HitActor (Collision|BreakHitResult _outhit)) (Game|GetPlayerCharacter 0)))
          (goto _label))))))

(fn ConstructionScript
  (|CallParentFunction))