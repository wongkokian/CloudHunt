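; Transform ring actor that switches control from the ALS player character to a Fish when the player overlaps its Plane.
; On overlap, it teleports the player to the world origin, zeroes the physics velocity of the first Fish found in the level and has player controller 0 possess it.
; Logic to move the Fish to the ring or trigger its jetstream movement is disconnected.
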(event OnComponentBeginOverlap(Plane)
  (params (OverlappedComponent :type Primitive%20Component%20Object%20Reference) (OtherActor :type Actor%20Object%20Reference) (OtherComp :type Primitive%20Component%20Object%20Reference) (OtherBodyIndex :type Integer) (bFromSweep :type Boolean) (SweepResult :type Hit%20Result%20Structure%20%28by%20ref%29))
  (bind _asals_player (Utilities|Casting|CastToALS_Player OtherActor))
  (bind _outactors (Actor|GetAllActorsOfClass "/Game/WaterElements/Fish.Fish_C"))
  (Transformation|Teleport _asals_player "0, 0, 0" "0, 0, 0")
  (Class|PrimitiveComponent|SetAllPhysicsLinearVelocity (Variables|/Script/Engine.DefaultPawn|GetMeshComponent (Utilities|Array|Get(acopy) _outactors)) "0, 0, 0" false)
  (Pawn|Possess (Game|GetPlayerController 0) (Utilities|Array|Get(acopy) _outactors)))

(event EventBeginPlay)

(event EventTick
  (params (DeltaSeconds :type Float%20%28single-precision%29)))

(fn ConstructionScript)