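; Phase controller for the Electric level's drivable car section, swapping the player between character and car.
; Triggering the phase shows and possesses the car and hides the character; completion ends the phase, re-possesses the character and unhides it.
; Sequencer events drive completion and target spawning through DriveableSpawner, which receives the car reference, supplies average accuracy and has its accuracy and beat reset at phase end.
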(event EventBeginPlay
  (CallFunction|Init))

(event Collision|EventActorBeginOverlap
  (params (OtherActor :type Actor%20Object%20Reference)))

(event EventTick
  (params (DeltaSeconds :type Float%20%28single-precision%29)))

(event Custom|Complete
  (Variables|Default|SetbFindCameraComponentWhenViewTarget true)
  (CallFunction|EndPhase)
  (Pawn|Possess (Game|GetPlayerController 0) (Variables|Default|GetPlayer%20Reference))
  (Rendering|SetActorHiddenInGame (Variables|Default|GetPlayer%20Reference) false))

(event Custom|Spawn%20Driveable%20Target
  (Default|SpawnTarget (Variables|Default|GetDriveableSpawner) 1.0))

(fn ConstructionScript)

(fn TriggerPhase
  (Rendering|SetActorHiddenInGame (Variables|Default|GetCar%20Reference) false)
  (Default|PossessCar (Variables|Default|GetCar%20Reference))
  (Rendering|SetActorHiddenInGame (Variables|Default|GetPlayer%20Reference) true)
  (|CallParentFunction))

(fn Init
  (Variables|Default|SetPlayer%20Reference (Game|GetPlayerCharacter 0))
  (Variables|/Game/Levels/ElectricLevel/Spawner/BP_DriveableSpawner.BP_DriveableSpawner_C|SetDriveableCar (Variables|Default|GetDriveableSpawner) (Variables|Default|GetCar%20Reference))
  (|CallParentFunction))

(fn GetAccuracy
  (bind _average_accuray (Default|GetAverageAccuracy (Variables|Default|GetDriveableSpawner)))
  (return _average_accuray))

(fn EndPhase
  (bind _driveablespawner (Variables|Default|GetDriveableSpawner))
  (|CallParentFunction)
  (Default|ResetAccuracy _driveablespawner)
  (Variables|/Game/Levels/ElectricLevel/Spawner/BP_DriveableSpawner.BP_DriveableSpawner_C|SetBeat _driveablespawner 0))