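; BP_DrivableRythmTarget is a rhythm target variant for the electric level that registers a hit through overlap, presumably when driven into.
; The first overlap on its Sphere component calls the inherited Hit function, guarded by a DoOnce.
; CalculateAccuracy returns a fixed near-perfect score instead of measuring timing.
; SetOffSet picks one of three lateral local-Y positions at random, but its call in the event graph is disconnected.
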(event OnComponentBeginOverlap(Sphere)
  (params (OverlappedComponent :type Primitive%20Component%20Object%20Reference) (OtherActor :type Actor%20Object%20Reference) (OtherComp :type Primitive%20Component%20Object%20Reference) (OtherBodyIndex :type Integer) (bFromSweep :type Boolean) (SweepResult :type Hit%20Result%20Structure%20%28by%20ref%29))
  (Utilities|FlowControl|DoOnce false
    (:Completed
      (CallFunction|Hit false))))

(event EventBeginPlay
  (|CallParentFunction))

(event Collision|EventActorBeginOverlap
  (params (OtherActor :type Actor%20Object%20Reference))
  (|CallParentFunction OtherActor) ; This node is disabled and will not be called.\nDrag off pins to build functionality.
)

(event EventTick
  (params (DeltaSeconds :type Float%20%28single-precision%29))
  (|CallParentFunction DeltaSeconds) ; This node is disabled and will not be called.\nDrag off pins to build functionality.
)

(fn ConstructionScript
  (|CallParentFunction))

(fn CalculateAccuracy
  (return 0.99))

(fn SetOffSet
  (Transformation|AddActorLocalOffset (Math|Vector|MakeVector 0.0 (Math|Conversions|ToFloat(Integer) (* (Math|Random|RandomIntegerinRange -1 1) 500)) 0.0) false false))