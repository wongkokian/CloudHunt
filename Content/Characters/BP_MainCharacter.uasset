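; Main player character Blueprint that adds a toggle crouch and a super jump triggered by Angel's Ladder actors.
; On BeginPlay it binds to the interaction component of every BP_AngelsLadder in the level.
; An active interaction applies a large upward impulse, gated by IsSuperjump.
; A free-running looping timer clears that flag periodically, so the cooldown varies with when the jump occurs.
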(event Custom|AngelsLadder_Hit
  (params (on :type Boolean))
  ;[1 1 1] AngelsLadder Super Jump
  (if on
    (if (not (Variables|Default|Getis_superjump))
      (Variables|Default|Setis_superjump true)
      (Physics|AddImpulse (Variables|Character|GetCharacterMovement) "0, 0,350000.000000" false))))

(event Custom|SuperJump_Reset%20Timer
  ;[1 1 1] AngelsLadder Super Jump
  (Variables|Default|Setis_superjump false))

(event EventBeginPlay
  (Utilities|FlowControl|Sequence
    (:then_0
      ;[1 1 1] AngelsLadder Super Jump
      (bind _outactors (Actor|GetAllActorsOfClass "/Game/GameElements/BP_AngelsLadder.BP_AngelsLadder_C"))
      (for _array_element _outactors
        (Utilities|IsValid (Actor|GetComponentbyClass _array_element "/Game/GameElements/BP_InteractionComponent.BP_InteractionComponent_C")
          (:Is%20Valid
            (EventDispatchers|BindEventtoOnInteraction (Actor|GetComponentbyClass _array_element "/Game/GameElements/BP_InteractionComponent.BP_InteractionComponent_C") (delegate Custom|AngelsLadder_Hit))))))
    (:then_1
      (Utilities|Time|SetTimerbyEvent (delegate Custom|SuperJump_Reset%20Timer) 1e+01 true))))

(event Input|ActionEvents|InputActionCrouch
  (params (Key :type Key%20Structure :default "None"))
  ;[1 1 1] Crouch
  (:Pressed
    (if (not (Variables|Default|GetbIsCrouched))
      (Character|Crouch)
      (else
        (Character|UnCrouch)))))

(fn ConstructionScript
  (|CallParentFunction))